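; GameManager actor that handles keyboard input for action modes and turn switching in what appears to be a grid-based tactics game.
; Keys set movement, attack or special mode flags and call ResetAllCube on the Vecteur actor with differing area flags.
; Space toggles the enemy turn, restores movement mode, resets the selected character and calls TurnChange on Vecteur.
; Input is enabled on BeginPlay, and mode changes print debug messages.
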(event `Key|Ampersand`
  (params (Key :type "Key Structure"))
  (:`Pressed`
    (`KismetSystemLibrary.PrintString` "Hello" :!label _label)))

(event `Key|E_AccentAigu`
  (params (Key :type "Key Structure"))
  (:`Pressed`
    (goto _label)))

(event `Key|E`
  (params (Key :type "Key Structure"))
  (:`Pressed`
    (set `self.IsMouvement` false)
    (set `self.IsSpecial` true)
    (`KismetSystemLibrary.PrintString` "Mode Special active")
    (bind _returnvalue (`GameplayStatics.GetActorOfClass` "/Game/Projet/Vecteur/Blueprint/Vecteur.Vecteur_C"))
    (`/Game/Projet/Vecteur/Blueprint/Vecteur.ResetAllCube` _returnvalue false true false)))

(event `Key|Z`
  (params (Key :type "Key Structure"))
  (:`Pressed`
    (set `self.IsMouvement` false)
    (set `self.IsSpecial` false)
    (`KismetSystemLibrary.PrintString` "Mode Attaque active")
    (bind _returnvalue (`GameplayStatics.GetActorOfClass` "/Game/Projet/Vecteur/Blueprint/Vecteur.Vecteur_C"))
    (`/Game/Projet/Vecteur/Blueprint/Vecteur.ResetAllCube` _returnvalue false true false)))

(event `Key|A`
  (params (Key :type "Key Structure"))
  (:`Pressed`
    (set `self.IsMouvement` true)
    (`KismetSystemLibrary.PrintString` "Mode Mouvement active")
    (bind _returnvalue (`GameplayStatics.GetActorOfClass` "/Game/Projet/Vecteur/Blueprint/Vecteur.Vecteur_C"))
    (`/Game/Projet/Vecteur/Blueprint/Vecteur.ResetAllCube` _returnvalue false false true)))

(event `Key|SpaceBar`
  (params (Key :type "Key Structure"))
  (:`Pressed`
    (bind _output_get (set `self.IsEnnemiTurn` (not (`self.IsEnnemiTurn`))))
    (`KismetSystemLibrary.PrintString` (`KismetStringLibrary.Concat_StrStr` "Tour de l'ennemi :" (`KismetStringLibrary.Conv_BoolToString` _output_get)))
    (set `self.IsMouvement` true)
    (set `self.IsSpecial` false)
    (set `self.SelectPerso` (`self.NULLPerso`))
    (bind _returnvalue (`GameplayStatics.GetActorOfClass` "/Game/Projet/Vecteur/Blueprint/Vecteur.Vecteur_C"))
    (`/Game/Projet/Vecteur/Blueprint/Vecteur.TurnChange` _returnvalue)))

(event `self.ReceiveBeginPlay`
  (`self.EnableInput` (`GameplayStatics.GetPlayerController` 0)))

(fn `UserConstructionScript`)