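; Perso is a character piece Blueprint that shows whether it is an enemy through the color of its Cone.
; SetColor applies the Red material when Ennemi is true and Blue otherwise, running from both the Construction Script and BeginPlay.
; A disconnected node that would place it just above its parent actor never runs, despite the comment describing that positioning.
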(event `self.ReceiveBeginPlay`
  ;[1 1 1] Défini la position du personnage à partir du cube dans lequel il est attaché et défini la couleur
  (`self.SetColor`))

(fn `SetColor`
  (if (`self.Ennemi`)
    (`PrimitiveComponent.SetMaterial` (`self.Cone`) 0 "/Game/Projet/Material/Red.Red")
    (else
      (`PrimitiveComponent.SetMaterial` (`self.Cone`) 0 "/Game/Projet/Material/Blue.Blue"))))

(fn `UserConstructionScript`
  (`self.SetColor`))