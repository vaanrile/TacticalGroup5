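; Perso_Controller provides helpers to identify and switch the character selected in GameManager among Automate, Char and Mecano (Ingenieur).
; Type checks compare the selected character's class with that of each placed actor of that type.
; Switch functions call GameManager's TabAction up to twice to cycle to the wanted type.
; It also returns an index for the current type, defaulting to Mecano, and the selected character's two cooldown wait times.
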(fn `CurrentPersoIs`
  (returns (ValPers :type Integer))
  (bind _isautomate (`self.InstanceOfAutomate`))
  (if _isautomate
    (return 0)
    (else
      (bind _ischar (`self.InstanceOfChar`))
      (if _ischar
        (return 1)
        (else
          (`self.InstanceOfMecano`)
          (return 2))))))

(fn `GetCdCurrentPerso`
  (returns (CdComp1 :type Integer) (CdComp2 :type Integer))
  (bind _returnvalue (`GameplayStatics.GetActorOfClass` "/Game/Projet/Blueprints/GameManager.GameManager_C"))
  (bind _selectperso (`/Game/Projet/Blueprints/GameManager.SelectPerso` _returnvalue))
  (`/Engine/EditorBlueprintResources/StandardMacros.IsValid` _selectperso
    (:`Is Valid`
      (return (`/Game/Projet/Blueprints/Perso.WaitTimeCDComp1` _selectperso) (`/Game/Projet/Blueprints/Perso.WaitTimeCDComp2` _selectperso)))
    (:`Is Not Valid`
      (return 0 0))))

(fn `InstanceOfAutomate`
  (returns (IsAutomate :type Boolean))
  (bind _returnvalue (`GameplayStatics.GetActorOfClass` "/Game/Projet/Blueprints/GameManager.GameManager_C"))
  (bind _outactors (`GameplayStatics.GetAllActorsOfClass` "/Game/Projet/Blueprints/Classe/Perso_Automate.Perso_Automate_C"))
  (for _array_element _outactors
    (if (== (`GameplayStatics.GetObjectClass` (`/Game/Projet/Blueprints/GameManager.SelectPerso` _returnvalue)) (`GameplayStatics.GetObjectClass` _array_element))
      (return true)))
  (return false))

(fn `InstanceOfChar`
  (returns (IsChar :type Boolean))
  (bind _returnvalue (`GameplayStatics.GetActorOfClass` "/Game/Projet/Blueprints/GameManager.GameManager_C"))
  (bind _outactors (`GameplayStatics.GetAllActorsOfClass` "/Game/Projet/Blueprints/Classe/Perso_Chars.Perso_Chars_C"))
  (for _array_element _outactors
    (if (== (`GameplayStatics.GetObjectClass` (`/Game/Projet/Blueprints/GameManager.SelectPerso` _returnvalue)) (`GameplayStatics.GetObjectClass` _array_element))
      (return true)))
  (return false))

(fn `InstanceOfMecano`
  (returns (IsAutomate :type Boolean))
  (bind _returnvalue (`GameplayStatics.GetActorOfClass` "/Game/Projet/Blueprints/GameManager.GameManager_C"))
  (bind _outactors (`GameplayStatics.GetAllActorsOfClass` "/Game/Projet/Blueprints/Classe/Perso_Ingenieur.Perso_Ingenieur_C"))
  (for _array_element _outactors
    (if (== (`GameplayStatics.GetObjectClass` (`/Game/Projet/Blueprints/GameManager.SelectPerso` _returnvalue)) (`GameplayStatics.GetObjectClass` _array_element))
      (return true)))
  (return false))

(fn `SwitchToAutomate`
  (bind _returnvalue (`GameplayStatics.GetActorOfClass` "/Game/Projet/Blueprints/GameManager.GameManager_C"))
  (bind _isautomate (`self.InstanceOfAutomate`))
  (if (not _isautomate)
    (`/Game/Projet/Blueprints/GameManager.TabAction` _returnvalue true)
    (bind _isautomate_2 (`self.InstanceOfAutomate`))
    (if (not _isautomate_2)
      (`/Game/Projet/Blueprints/GameManager.TabAction` _returnvalue true))))

(fn `SwitchToChar`
  (bind _returnvalue (`GameplayStatics.GetActorOfClass` "/Game/Projet/Blueprints/GameManager.GameManager_C"))
  (bind _ischar (`self.InstanceOfChar`))
  (if (not _ischar)
    (`/Game/Projet/Blueprints/GameManager.TabAction` _returnvalue true)
    (bind _ischar_2 (`self.InstanceOfChar`))
    (if (not _ischar_2)
      (`/Game/Projet/Blueprints/GameManager.TabAction` _returnvalue true))))

(fn `SwitchToMecano`
  (bind _returnvalue (`GameplayStatics.GetActorOfClass` "/Game/Projet/Blueprints/GameManager.GameManager_C"))
  (bind _isautomate (`self.InstanceOfMecano`))
  (if (not _isautomate)
    (`/Game/Projet/Blueprints/GameManager.TabAction` _returnvalue true)
    (bind _isautomate_2 (`self.InstanceOfMecano`))
    (if (not _isautomate_2)
      (`/Game/Projet/Blueprints/GameManager.TabAction` _returnvalue true))))

(fn `UserConstructionScript`)