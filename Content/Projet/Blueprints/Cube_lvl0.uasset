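; Cube_lvl0 is a tile actor that overheats in stages and damages the referenced character (Personage) once fully heated.
; Successive WillBurn calls raise the Surchauffe level, turning Tile1 red at the first stage.
; At the top level, each further call damages Personage through RecoitDegat, if valid, and restarts a short burn timer.
; Tick runs SurchauffeFonction during a burn to count down and show, then hide, the fire particle.
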(event `self.ReceiveTick`
  (params (DeltaSeconds :type "Float (single-precision)"))
  (if (`self.IsAnimBurning`)
    (`self.SurchauffeFonction` DeltaSeconds))
  (`parent.ReceiveTick` DeltaSeconds))

(fn `SurchauffeFonction`
  (params (`Delta Time` :type "Float (double-precision)"))
  (bind _output_get (set `self.surchauffeTime` (- (`self.surchauffeTime`) `Delta Time`)))
  (bind _returnvalue (> _output_get 0.0))
  (if _returnvalue
    (`SceneComponent.SetVisibility` (`self.Fireparticule`) _returnvalue false)
    (else
      (set `self.IsAnimBurning` false)
      (`SceneComponent.SetVisibility` (`self.Fireparticule`) false false))))

(fn `UserConstructionScript`
  (`parent.UserConstructionScript`))

(fn `WillBurn`
  (bind _personage (`self.Personage`))
  (if (== (`self.Surchauffe`) 0)
    (set `self.Surchauffe` 1)
    (`PrimitiveComponent.SetMaterial` (`self.tile1`) 0 "/Game/Projet/Character/Material_Red/MainRed.MainRed")
    (elif (== (`self.Surchauffe`) 1)
      (set `self.Surchauffe` 2)
      (elif (== (`self.Surchauffe`) 2)
        (`/Engine/EditorBlueprintResources/StandardMacros.IsValid` _personage
          (:`Is Valid`
            (set `self.IsAnimBurning` true)
            (set `self.surchauffeTime` 2.0)
            (`/Game/Projet/Blueprints/Perso.RecoitDegat` _personage 2.0)))))))