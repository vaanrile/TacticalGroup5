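; Grid manager for a turn-based tactics game, mapping cubes to 2D coordinates and placing characters on them.
; At BeginPlay it derives coordinates from world positions into a cube dictionary.
; CreateArea flood-fills move, attack and toggled enemy-threat areas, storing paths per cube and weighing diagonals, height, barriers and occupants.
; Turn changes clear highlights and heat a growing share of shuffled level-0 cubes toward burning, with sound events.
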(event `self.ReceiveTick`
  (params (DeltaSeconds :type "Float (single-precision)"))
  (if (`self.One Perso Burn`)
    (bind _output_get (set `self.WaitTime` (- (`self.WaitTime`) 1)))
    (if (< _output_get 0)
      (`FMODBlueprintStatics.PlayEvent2D` "/Game/FMOD/Events/Environment_SFX/Tile_Burn.Tile_Burn")
      (set `self.One Perso Burn` false))))

(event `TurnChange`
  (params (Turn :type Integer))
  (`KismetArrayLibrary.Array_Clear` (`self.SelectEnnemi`))
  (`self.ResetAllCube` true true true true)
  (`self.Burn Case` Turn))

(event `OnCreationAttackArea`
  (params (Cube :type "/Game/Projet/Blueprints/Cube Object Reference"))
  (`self.Create Area` (`/Game/Projet/Blueprints/Perso.AttackRange` (`/Game/Projet/Blueprints/Cube.Personage` Cube)) Cube false false true))

(event `CheckEnnemiRadius`
  (params (PersoClick :type "/Game/Projet/Blueprints/Cube Object Reference"))
  (bind _selectennemi (`self.SelectEnnemi`))
  ;[1 1 1] Vérifie si le cube sélectionné est dans la liste
  (if (`KismetArrayLibrary.Array_Contains` _selectennemi PersoClick)
    ;[1 1 1] Enlève
    (`KismetArrayLibrary.Array_RemoveItem` _selectennemi PersoClick)
    (else
      ;[1 1 1] Ajoute
      (`KismetArrayLibrary.Array_AddUnique` _selectennemi PersoClick)))
  ;[1 1 1] Réinitialise la zone d'ennemi
  (`self.ResetAllCube` true false false true)
  ;[1 1 1] Recréer la zone d'ennemi
  (for _array_element (`self.SelectEnnemi`)
    (`self.Create Area` (`/Game/Projet/Blueprints/Perso.NumberMove` (`/Game/Projet/Blueprints/Cube.Personage` _array_element)) _array_element true false false true)
    (`self.ResetAllCube` false false false true)))

(event `OnMovePerso`
  (bind _selectcube (`self.SelectCube`))
  (bind _selectcube_2 (`self.SelectCube`))
  (bind _returnvalue (`GameplayStatics.GetActorOfClass` "/Game/Projet/Blueprints/GameManager.GameManager_C"))
  (bind _selectperso (`/Game/Projet/Blueprints/GameManager.SelectPerso` _returnvalue))
  (`self.K2_AttachToActor` _selectperso _selectcube "None" "KeepRelative" "KeepRelative" "KeepRelative" true)
  (`self.K2_SetActorLocation` _selectperso (+ (`self.K2_GetActorLocation` _selectcube) (0.0 0.0 50.0)) false false)
  (bind _returnvalue_2 (`GameplayStatics.GetActorOfClass` "/Game/Projet/Blueprints/GameManager.GameManager_C"))
  (bind _selectperso_2 (`/Game/Projet/Blueprints/GameManager.SelectPerso` _returnvalue_2))
  (set `/Game/Projet/Blueprints/Cube.Personage` _selectperso_2 _selectcube_2)
  (set `/Game/Projet/Blueprints/Perso.MyCube` _selectcube_2 _selectperso_2)
  (`/Game/Projet/Blueprints/Perso.ZoneMovePerso` _selectperso_2))

(event `OnClickCube`
  (params (CubeSelect :type "/Game/Projet/Blueprints/Cube Object Reference") (NombreMouvement :type "Float (double-precision)"))
  (`self.ResetAllCube` false true)
  (`self.Create Area` NombreMouvement CubeSelect false true false true))

(event `self.ReceiveBeginPlay`
  ;[1 1 1] Set information for all the cube about a 2D vector
  ;;[1 1 1] Positionne l'objet dans le cube parent
  (`self.K2_SetActorLocation` (`self.K2_GetActorLocation` (`self.GetAttachParentActor`)))
  ;;[1 1 1] Défini les variables vecteurs dans tous les cubes
  (bind _outactors (`GameplayStatics.GetAllActorsOfClass` "/Game/Projet/Blueprints/Cube.Cube_C"))
  (`self.SetVectorXY` _outactors)
  ;;[1 1 1] Initialize dictionnary
  (for _array_element _outactors
    (`SceneComponent.SetRelativeScale3D` (`/Game/Projet/Blueprints/Cube.Cube` _array_element) (0.9 0.9 1.1))
    (`BlueprintMapLibrary.Map_Add` (`self.CubeDictionnary`) (make `IntVector` (`/Game/Projet/Blueprints/Cube.VectorX` _array_element) (`/Game/Projet/Blueprints/Cube.VectorY` _array_element)) _array_element))
  (bind _outactors_2 (`GameplayStatics.GetAllActorsOfClass` "/Game/Projet/Blueprints/Perso.Perso_C"))
  (`self.SetPersoLocation` _outactors_2)
  (bind _outactors_3 (`GameplayStatics.GetAllActorsOfClass` "/Game/Projet/Blueprints/Cube_lvl0.Cube_lvl0_C"))
  (bind _output_get (set `self.TabCubeCanBurn` _outactors_3))
  (`KismetArrayLibrary.Array_Shuffle` _output_get))

(fn `AllPersoRecoitTmpDegat`
  (bind _outactors (`GameplayStatics.GetAllActorsOfClass` "/Game/Projet/Blueprints/Perso.Perso_C"))
  (for _array_element _outactors
    (if (`/Game/Projet/Blueprints/Perso.IsRobot` _array_element)
      (`/Game/Projet/Blueprints/Perso.RecoitTmpDegat` _array_element))))

(fn `AnalyseIfPersoInCube`
  (bind _output_get (set `self.SelectCube` null)))

(fn `Burn Case`
  (params (Turn :type Integer))
  (locals (IsOneWillBurn :type Boolean))
  (bind _returnvalue (`KismetArrayLibrary.Array_Length` (`self.TabCubeCanBurn`)))
  (bind _returnvalue_2 (* (- Turn 2) 10))
  (if (> _returnvalue _returnvalue_2)
    (for _index (range (+ _returnvalue_2 1))
      (bind _output (`|GetArrayItem` (`self.TabCubeCanBurn`) _index))
      (bind _onepersoburn (`/Game/Projet/Blueprints/Cube.WillBurn` _output))
      (set `local.IsOneWillBurn` (== (`/Game/Projet/Blueprints/Cube.Surchauffe` _output) 1))
      (set `self.One Perso Burn` _onepersoburn))
    (else
      (for _index_2 (range _returnvalue)
        (bind _output_2 (`|GetArrayItem` (`self.TabCubeCanBurn`) _index_2))
        (bind _onepersoburn_2 (`/Game/Projet/Blueprints/Cube.WillBurn` _output_2))
        (set `local.IsOneWillBurn` (== (`/Game/Projet/Blueprints/Cube.Surchauffe` _output_2) 1))
        (set `self.One Perso Burn` _onepersoburn_2))))
  (if (`local.IsOneWillBurn`)
    (`FMODBlueprintStatics.PlayEvent2D` "/Game/FMOD/Events/Environment_SFX/Tile_Heat.Tile_Heat")
    (if (`self.One Perso Burn`)
      (set `self.WaitTime` 10))))

(fn `Create Area`
  (params (NumberMove :type "Float (double-precision)") (Origin :type "/Game/Projet/Blueprints/Cube Object Reference") (AreaEnnemiMove :type Boolean) (AreaMove :type Boolean) (AreaAttack :type Boolean) (ObstacleDetection :type Boolean))
  (locals (UseCube :type "Array of /Game/Projet/Blueprints/Cube Object Reference") (StockCube :type "Array of /Game/Projet/Blueprints/Cube Object Reference") (TempOffset :type "Array of Vector Structure") (MoveCase :type "Float (double-precision)"))
  (bind _usecube (`local.UseCube`))
  (bind _stockcube (`local.StockCube`))
  (bind _areamove (`local.AreaMove`))
  (bind _origin (`local.Origin`))
  ;[1 1 1] Reset les cases move
  (`self.ResetAllCube` false false false true)
  ;[1 1 1] Ajout dans la file le cube d'origine
  (`KismetArrayLibrary.Array_AddUnique` (`local.UseCube`) Origin)
  ;[1 1 1] Vérifie la zone centrale à colorer
  (if (`local.AreaMove`)
    (set `/Game/Projet/Blueprints/Cube.AllierMoveArea` true _origin)
    (set `/Game/Projet/Blueprints/Cube.MoveRange` NumberMove _origin :!label _label)
    ;[1 1 1] Ajoute dans la variable du pathfinding le cube d'origine
    (`KismetArrayLibrary.Array_AddUnique` (`/Game/Projet/Blueprints/Cube.PathCube` _origin) _origin)
    ;[1 1 1] Boucle en fonction de la portée
    (for _ (range (+ (`KismetMathLibrary.FTrunc` NumberMove) 1))
      ;[1 1 1] Boucle en fonction des données dans la file
      (for _array_element _usecube
        ;[1 1 1] Boucle pour chercher les cases adjacents
        (for _array_element_2 (`local.TempOffset`)
          (bind _returnvalue (`KismetMathLibrary.FTrunc` (.x _array_element_2)))
          (bind _returnvalue_2 (`KismetMathLibrary.FTrunc` (.y _array_element_2)))
          ;[1 1 1] Analyse des cases adjacentes
          (if (or (== _returnvalue 0) (== _returnvalue_2 0))
            (set `local.MoveCase` 0.0)
            (else
              (set `local.MoveCase` (`self.CoeffDiago`))))
          (bind _cube (`self.GetCubeAtGridPosition` (+ _returnvalue (`/Game/Projet/Blueprints/Cube.VectorX` _array_element)) (+ _returnvalue_2 (`/Game/Projet/Blueprints/Cube.VectorY` _array_element))))
          (`/Engine/EditorBlueprintResources/StandardMacros.IsValid` _cube
            (:`Is Valid`
              (if (and _areamove (!= (`/Game/Projet/Blueprints/Cube.Hauteur` _cube) (`/Game/Projet/Blueprints/Cube.Hauteur` _array_element)))
                (set `local.MoveCase` (+ (`local.MoveCase`) 0.5)))
              (if (`local.ObstacleDetection`)
                (if (not (>= (- (`/Game/Projet/Blueprints/Cube.Hauteur` _cube) (`/Game/Projet/Blueprints/Cube.Hauteur` _array_element)) 2))
                  (`/Engine/EditorBlueprintResources/StandardMacros.IsValid` (`/Game/Projet/Blueprints/Cube.Personage` _cube)
                    (:`Is Not Valid`
                      (bind _returnvalue_3 (- (`/Game/Projet/Blueprints/Cube.MoveRange` _array_element) (`local.MoveCase`)))
                      (if (>= _returnvalue_3 (+ (`/Game/Projet/Blueprints/Cube.MoveRange` _cube) 1.0)) :!label _label_2
                        (if (>= _returnvalue_3 0.0)
                          (if _areamove
                            (if (`/Game/Projet/Blueprints/Cube.isBarriere` _cube)
                              (set `local.MoveCase` (+ (`local.MoveCase`) 0.5))
                              (else
                                (set `/Game/Projet/Blueprints/Cube.AllierMoveArea` true _cube)))
                            (set `/Game/Projet/Blueprints/Cube.MoveRange` (- _returnvalue_3 1.0) _cube :!label _label_3)
                            (bind _pathcube (`/Game/Projet/Blueprints/Cube.PathCube` _cube))
                            (`KismetArrayLibrary.Array_Clear` _pathcube)
                            (`KismetArrayLibrary.Array_Append` _pathcube (`/Game/Projet/Blueprints/Cube.PathCube` _array_element))
                            (`KismetArrayLibrary.Array_AddUnique` _pathcube _cube)
                            (`KismetArrayLibrary.Array_AddUnique` (`local.StockCube`) _cube)
                            (if (`/Game/Projet/Blueprints/Cube.CursorOverIt` _cube)
                              (`/Game/Projet/Blueprints/Cube.PathFindingMove` _cube))
                            (elif (`local.AreaAttack`)
                              (set `/Game/Projet/Blueprints/Cube.AllierAttackArea` true _cube)
                              (goto _label_3)
                              (elif (`local.AreaEnnemiMove`)
                                (set `/Game/Projet/Blueprints/Cube.EnnemiAttackArea` true _cube)
                                (goto _label_3)))))))))
                (else
                  (goto _label_2)))))))
      ;[1 1 1] Stockage des données dans la file
      (`KismetArrayLibrary.Array_Clear` _usecube)
      (`KismetArrayLibrary.Array_Append` _usecube _stockcube)
      (`KismetArrayLibrary.Array_Clear` _stockcube))
    (elif (`local.AreaAttack`)
      (set `/Game/Projet/Blueprints/Cube.AllierAttackArea` true _origin)
      (goto _label)
      (elif (`local.AreaEnnemiMove`)
        (set `/Game/Projet/Blueprints/Cube.EnnemiAttackArea` true _origin)
        (goto _label)))))

(fn `GetCubeAtGridPosition`
  (params (x :type Integer) (y :type Integer))
  (returns (Cube :type "/Game/Projet/Blueprints/Cube Object Reference"))
  (return (`BlueprintMapLibrary.Map_Find` (`self.CubeDictionnary`) (make `IntVector` x y))))

(fn `GetCubeFromPerso`
  (params (ListPerso :type "/Game/Projet/Blueprints/Perso Object Reference"))
  (returns (RecupCube :type "/Game/Projet/Blueprints/Cube Object Reference"))
  (bind (_returnvalue_x _returnvalue_y) (`KismetMathLibrary.BreakVector` (`self.K2_GetActorLocation` ListPerso)))
  (bind (_returnvalue_x_2 _returnvalue_y_2) (`KismetMathLibrary.BreakVector` (`self.K2_GetActorLocation`)))
  (bind _cubedictionnary (`self.CubeDictionnary`))
  (bind (_returnvalue_x_3 _returnvalue_y_3) (`KismetMathLibrary.BreakVector` (`SceneComponent.K2_GetComponentScale` (`Actor.RootComponent` ListPerso))))
  (bind (_min _max) (`StaticMeshComponent.GetLocalBounds` (`/Game/Projet/Blueprints/Perso.Cone` ListPerso)))
  (bind _returnvalue (`self.CalculVector` _returnvalue_y _returnvalue_y_2 (* _returnvalue_y_3 (- (.y _max) (.y _min)))))
  (bind _returnvalue_2 (* (`self.CalculVector` _returnvalue_x _returnvalue_x_2 (* (* _returnvalue_x_3 (- (.x _max) (.x _min))) -1.0)) -1))
  (if (`BlueprintMapLibrary.Map_Contains` _cubedictionnary (make `IntVector` _returnvalue_2 _returnvalue))
    (return (`BlueprintMapLibrary.Map_Find` _cubedictionnary (make `IntVector` _returnvalue_2 _returnvalue)))
    (else
      (`KismetSystemLibrary.PrintString` "Hello"))))

(fn `ResetAllCube`
  (params (IsAreaEnnemiMove :type Boolean) (IsAllierAreaMove :type Boolean) (IsAllierAreaAttack :type Boolean) (isNumberMove :type Boolean))
  (locals (IsAreaEnnemiMoveVar :type Boolean) (IsAllierAreaMoveVar :type Boolean) (IsAllierAreaAttackVar :type Boolean))
  (set `local.IsAreaEnnemiMoveVar` IsAreaEnnemiMove)
  (set `local.IsAllierAreaMoveVar` IsAllierAreaMove)
  (set `local.IsAllierAreaAttackVar` IsAllierAreaAttack)
  (bind _outactors (`GameplayStatics.GetAllActorsOfClass` "/Game/Projet/Blueprints/Cube.Cube_C"))
  (for _array_element _outactors
    (if isNumberMove
      (set `/Game/Projet/Blueprints/Cube.MoveRange` 0.0 _array_element)
      (`KismetArrayLibrary.Array_Clear` (`/Game/Projet/Blueprints/Cube.PathCube` _array_element))
      (if (not (`/Game/Projet/Blueprints/Cube.CursorOverIt` _array_element))
        (set `/Game/Projet/Blueprints/Cube.Highlighted` false _array_element)))
    (if (`local.IsAreaEnnemiMoveVar`)
      (set `/Game/Projet/Blueprints/Cube.EnnemiAttackArea` false _array_element))
    (if (`local.IsAllierAreaMoveVar`)
      (set `/Game/Projet/Blueprints/Cube.AllierMoveArea` false _array_element))
    (if (`local.IsAllierAreaAttackVar`)
      (set `/Game/Projet/Blueprints/Cube.AllierAttackArea` false _array_element))))

(fn `SetPersoLocation`
  (params (ListPerso :type "Array of /Game/Projet/Blueprints/Perso Object Reference"))
  (for _array_element ListPerso
    (`/Game/Projet/Blueprints/Perso.InitStat` _array_element)
    (bind _mycube (`/Game/Projet/Blueprints/Perso.MyCube` _array_element))
    (bind _output_get (set `/Game/Projet/Blueprints/Cube.Personage` _array_element _mycube))
    (`self.K2_AttachToActor` _array_element _mycube "None" "KeepRelative" "KeepRelative" "KeepRelative" true)
    (`self.K2_SetActorLocation` _output_get (+ (`SceneComponent.K2_GetComponentLocation` (`/Game/Projet/Blueprints/Cube.DefaultSceneRoot` _mycube)) (0.0 0.0 50.0)) false false))
  (bind _returnvalue (`GameplayStatics.GetActorOfClass` "/Game/Projet/Blueprints/GameManager.GameManager_C"))
  (`/Game/Projet/Blueprints/GameManager.Init HB UI` _returnvalue))

(fn `SetVectorXY`
  (params (Array :type "Array of /Game/Projet/Blueprints/Cube Object Reference"))
  (bind (_returnvalue_x _returnvalue_y _returnvalue_z) (`KismetMathLibrary.BreakVector` (`self.K2_GetActorLocation`)))
  ;[1 1 1] Boucle qui compare les positions des cubes afin d'y mettre les coordonées de vecteurs 2D
  (for _array_element Array
    (bind (_returnvalue_x_2 _returnvalue_y_2 _returnvalue_z_2) (`KismetMathLibrary.BreakVector` (`self.K2_GetActorLocation` _array_element)))
    (bind (_returnvalue_x_3 _returnvalue_y_3 _returnvalue_z_3) (`KismetMathLibrary.BreakVector` (`SceneComponent.K2_GetComponentScale` (`/Game/Projet/Blueprints/Cube.Cube` _array_element))))
    (bind (_min _max) (`StaticMeshComponent.GetLocalBounds` (`/Game/Projet/Blueprints/Cube.Cube` _array_element)))
    (set `/Game/Projet/Blueprints/Cube.VectorX` (* (`self.CalculVector` _returnvalue_x_2 _returnvalue_x (* (* _returnvalue_x_3 (- (.x _max) (.x _min))) -1.0)) -1) _array_element)
    (set `/Game/Projet/Blueprints/Cube.VectorY` (`self.CalculVector` _returnvalue_y_2 _returnvalue_y (* _returnvalue_y_3 (- (.y _max) (.y _min)))) _array_element)))

(fn `UserConstructionScript`)