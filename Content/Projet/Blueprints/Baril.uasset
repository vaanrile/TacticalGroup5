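; Baril is an explosive barrel on a tactical grid, placed on a cube by its number with stats from a barrel struct.
; On death it frees its cube and runs PushExplosion along each direction, stacking robots and debris to shove.
; Obstacles add impact damage, and barrels met en route damage units in range and are destroyed.
; Pushed units get new cubes and push targets, then the Vecteur grid actor applies accumulated damage.
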(event `self.ReceiveBeginPlay`
  (`parent.ReceiveBeginPlay`)
  (`self.InitStat`)
  (set `self.IsRobot` false))

(fn `Death`
  (locals (dirs :type "Array of Vector Structure") (Init :type "Vector Structure"))
  (bind _mycube (`self.MyCube`))
  (set `/Game/Projet/Blueprints/Cube.Personage` null _mycube)
  (bind _output_get (set `local.Init` (`KismetMathLibrary.MakeVector` (`KismetMathLibrary.Conv_IntToDouble` (`/Game/Projet/Blueprints/Cube.VectorX` _mycube)) (`KismetMathLibrary.Conv_IntToDouble` (`/Game/Projet/Blueprints/Cube.VectorY` _mycube)))))
  (for _array_element (`local.dirs`)
    (`self.PushExplosion` _array_element _output_get))
  (`parent.Death`))

(fn `GetPersoInRange`
  (returns (ListPersoVoisin :type "Array of /Game/Projet/Blueprints/Perso Object Reference"))
  (locals (TmpListPerso :type "Array of /Game/Projet/Blueprints/Perso Object Reference"))
  (bind _mycube (`self.MyCube`))
  (bind _returnvalue (`KismetMathLibrary.FTrunc` (`self.AttackRange`)))
  (bind _returnvalue_2 (* _returnvalue -1))
  (bind _returnvalue_3 (`GameplayStatics.GetActorOfClass` "/Game/Projet/Blueprints/Vecteur.Vecteur_C"))
  ;[1 1 1] Double boucle pour checker le voisinage
  (for _index (range _returnvalue_2 (+ _returnvalue 1))
    (for _index_2 (range _returnvalue_2 (+ _returnvalue 1))
      (if (not (and (== _index 0) (== _index_2 0)))
        (bind _cube (`/Game/Projet/Blueprints/Vecteur.GetCubeAtGridPosition` _returnvalue_3 (+ (`/Game/Projet/Blueprints/Cube.VectorX` _mycube) _index) (+ (`/Game/Projet/Blueprints/Cube.VectorY` _mycube) _index_2)))
        (`/Engine/EditorBlueprintResources/StandardMacros.IsValid` _cube
          (:`Is Valid`
            (bind _personage (`/Game/Projet/Blueprints/Cube.Personage` _cube))
            (`/Engine/EditorBlueprintResources/StandardMacros.IsValid` _personage
              (:`Is Valid`
                (`KismetArrayLibrary.Array_Add` (`local.TmpListPerso`) _personage))))))))
  (return (`local.TmpListPerso`)))

(fn `InitStat`
  (bind _numbercube (`self.NumberCube`))
  (bind (_attackrange _attackdamage _hp _posxb1 _posyb1 _posxb2 _posyb2 _posxb3 _posyb3 _posxb4 _posxb5) (break `/Game/Projet/Structure/Structure_Baril` (make `/Game/Projet/Structure/Structure_Baril` 1.0)))
  (bind _returnvalue (`GameplayStatics.GetActorOfClass` "/Game/Projet/Blueprints/Vecteur.Vecteur_C"))
  (set `self.AttackRange` _attackrange)
  (set `self.AttackDamage` _attackdamage)
  (set `self.LifePoint` _hp)
  (if (== _numbercube 1)
    (bind _cube (`/Game/Projet/Blueprints/Vecteur.GetCubeAtGridPosition` _returnvalue _posxb1 _posyb1))
    (set `self.MyCube` _cube)
    (elif (== _numbercube 2)
      (bind _cube_2 (`/Game/Projet/Blueprints/Vecteur.GetCubeAtGridPosition` _returnvalue _posxb2 _posyb2))
      (set `self.MyCube` _cube_2)
      (elif (== _numbercube 3)
        (bind _cube_3 (`/Game/Projet/Blueprints/Vecteur.GetCubeAtGridPosition` _returnvalue _posxb3 _posyb3))
        (set `self.MyCube` _cube_3)
        (else
          (bind _cube_4 (`/Game/Projet/Blueprints/Vecteur.GetCubeAtGridPosition` _returnvalue _posxb4 _posxb5))
          (set `self.MyCube` _cube_4)))))
  (`parent.InitStat`))

(fn `PushExplosion`
  (params (Dir :type "Vector Structure") (PosInit :type "Vector Structure"))
  (locals (VecteurDirection :type "Vector Structure") (VecteurTemp :type "Vector Structure") (PilePerso :type "Array of /Game/Projet/Blueprints/Perso Object Reference") (NonObstacle :type Boolean :default true) (Max :type "Float (double-precision)" :default 1.0) (Compteur1 :type Integer) (NonObstacle :type Boolean) (ListpersoTMP :type "Array of /Game/Projet/Blueprints/Perso Object Reference"))
  (bind (_vecteurtemp_x _vecteurtemp_y) (`KismetMathLibrary.BreakVector` (`local.VecteurTemp`)))
  (bind _pileperso (`local.PilePerso`))
  (bind (_vecteurtemp_x_2 _vecteurtemp_y_2 _vecteurtemp_z) (`KismetMathLibrary.BreakVector` (`local.VecteurTemp`)))
  (bind _output (`|GetArrayItem` _pileperso (`KismetArrayLibrary.Array_LastIndex` _pileperso)))
  (set `local.VecteurDirection` Dir)
  (set `local.VecteurTemp` PosInit)
  (set `local.Max` 1.0)
  (bind _returnvalue (`GameplayStatics.GetActorOfClass` "/Game/Projet/Blueprints/Vecteur.Vecteur_C"))
  ;[1 1 1] Boucle qui vérifie si on ne recontre pas d'obstacle ou si on ne dépasse pas la portée de charge
  (while (and (`local.NonObstacle`) (< (`local.Compteur1`) (`KismetMathLibrary.FTrunc` (`local.Max`))))
    (`KismetSystemLibrary.PrintString` "Hello")
    ;[1 1 1] Incrémentation de vecteur temporaire à partir de la direction
    (bind _output_get (set `local.VecteurTemp` (+ (`local.VecteurDirection`) (`local.VecteurTemp`))))
    ;[1 1 1] Récupération du cube
    (bind _cube (`/Game/Projet/Blueprints/Vecteur.GetCubeAtGridPosition` _returnvalue (`KismetMathLibrary.FTrunc` (.x _output_get)) (`KismetMathLibrary.FTrunc` (.y _output_get))))
    ;[1 1 1] Vérifie s'il rencontre des obstacles
    (`/Engine/EditorBlueprintResources/StandardMacros.IsValid` _cube
      (:`Is Valid`
        (if (> (`KismetMathLibrary.Conv_IntToDouble` (`/Game/Projet/Blueprints/Cube.Hauteur` _cube)) _vecteurtemp_z)
          (set `local.NonObstacle` false :!label _label)
          (elif (`/Game/Projet/Blueprints/Cube.isBarriere` _cube)
            (goto _label)
            (else
              (bind _personage (`/Game/Projet/Blueprints/Cube.Personage` _cube))
              ;[1 1 1] Personnage ?
              (`/Engine/EditorBlueprintResources/StandardMacros.IsValid` _personage
                (:`Is Valid`
                  ;[1 1 1] Baril ou robot ?
                  (if (`/Game/Projet/Blueprints/Perso.IsRobot` _personage)
                    ;[1 1 1] Ajoute +1 à max et ajoute le perso dans la pile
                    (set `local.Max` (+ (`local.Max`) 1.0) :!label _label_2)
                    (`KismetArrayLibrary.Array_AddUnique` (`local.PilePerso`) _personage)
                    (else
                      ;[1 1 1] Cast le baril
                      (bind _asbaril (cast `/Game/Projet/Blueprints/Baril` _personage)
                        (:`then`
                          ;[1 1 1] Vide la liste des personnages qui prendront les dégâts du barils (au cas ou 2 barils sont chargés)
                          (`KismetArrayLibrary.Array_Clear` (`local.ListpersoTMP`))
                          ;[1 1 1] Ajoute à la liste les personnages a portée de l'explosion du baril
                          (bind _listpersovoisin (`self.GetPersoInRange` _asbaril))
                          (for _array_element _listpersovoisin
                            (`KismetArrayLibrary.Array_AddUnique` (`local.ListpersoTMP`) _array_element))
                          ;[1 1 1] Si il y a des personnages dans la pile, certains sont à portée de l'explosion quand ils sont poussés. Ajouté de manière unique pour eviter qu'un personnage prenne deux fois les dégâts
                          (for (_array_element_2 _array_index) (`local.PilePerso`)
                            (if (<= _array_index (`KismetMathLibrary.FTrunc` (`/Game/Projet/Blueprints/Perso.AttackRange` _asbaril)))
                              (`KismetArrayLibrary.Array_AddUnique` (`local.ListpersoTMP`) _array_element_2)
                              (else
                                (break))))
                          ;[1 1 1] Inflige les dégâts du baril
                          (for _array_element_3 (`local.ListpersoTMP`)
                            (`self.AccumulDegat` _array_element_3 (`/Game/Projet/Blueprints/Perso.AttackDamage` _asbaril)))
                          ;[1 1 1] Détruit le baril
                          (`self.K2_DestroyActor` _asbaril))
                        (:`CastFailed`
                          (cast `/Game/Projet/Blueprints/Debris` _personage)
                          (goto _label_2))))))
                (:`Is Not Valid`
                  _))
              ;[1 1 1] +1 au compteur
              (set `local.Compteur1` (+ (`local.Compteur1`) 1))))))
      (:`Is Not Valid`
        (goto _label))))
  ;[1 1 1] Test si un obstacle a été rencontré
  (if (not (`local.NonObstacle`))
    ;[1 1 1] Obstacle rencontré, le dernier subit les dégâts du mur et on recule le vecteur pour eviter de mettre un personnage dans un mur
    (`/Engine/EditorBlueprintResources/StandardMacros.IsValid` _output
      (:`Is Valid`
        (`self.AccumulDegat` _output 2.0)
        (set `local.VecteurTemp` (- (`local.VecteurTemp`) (`local.VecteurDirection`))))
      (:`Is Not Valid`
        _)))
  ;[1 1 1] Permet de recuperer le perso Null
  (bind _returnvalue_2 (`GameplayStatics.GetActorOfClass` "/Game/Projet/Blueprints/GameManager.GameManager_C"))
  ;[1 1 1] Depile de la pile charge
  (bind (_arrayindex _arrayelement) (`/Engine/EditorBlueprintResources/StandardMacros.ReverseForEachLoop` (`local.PilePerso`))
    (:`LoopBody`
      (if (== _arrayindex 0)
        (`self.AccumulDegat` _arrayelement 2.0))
      (bind _mycube (`/Game/Projet/Blueprints/Perso.MyCube` _arrayelement))
      (set `/Game/Projet/Blueprints/Cube.Personage` (`/Game/Projet/Blueprints/GameManager.NULLPerso` _returnvalue_2) _mycube)
      (bind _cube_2 (`/Game/Projet/Blueprints/Vecteur.GetCubeAtGridPosition` _returnvalue (`KismetMathLibrary.FTrunc` _vecteurtemp_x) (`KismetMathLibrary.FTrunc` _vecteurtemp_y)))
      (set `/Game/Projet/Blueprints/Perso.TargetPushCube` _cube_2 _arrayelement)
      (set `/Game/Projet/Blueprints/Perso.DerHauteur` (`/Game/Projet/Blueprints/Cube.Hauteur` _mycube) _arrayelement)
      (set `/Game/Projet/Blueprints/Cube.Personage` _arrayelement _cube_2)
      (set `/Game/Projet/Blueprints/Perso.MyCube` _cube_2 _arrayelement)
      (set `/Game/Projet/Blueprints/Perso.WhereIsPush` (`self.K2_GetActorLocation` _cube_2) _arrayelement)
      (set `/Game/Projet/Blueprints/Perso.IsPushed` true _arrayelement)
      ;;[1 1 1] déplace la position cible
      (set `local.VecteurTemp` (- (`local.VecteurTemp`) (`local.VecteurDirection`))))
    (:`Completed`
      ;[1 1 1] inflige les dégats
      (`/Game/Projet/Blueprints/Vecteur.AllPersoRecoitTmpDegat` _returnvalue))))

(fn `Set Color`
  (`PrimitiveComponent.SetMaterial` (`self.Cone`) 0 "/Game/Projet/Material/Burn.Burn"))

(fn `UserConstructionScript`)