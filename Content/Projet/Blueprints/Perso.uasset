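; Base tactical grid character, player or enemy, with team-colored cone, health bar, movement allowance and one attack flag.
; Movement, attack and skill zones are delegated to the Vecteur grid actor, with characters attached to cubes.
; Attacks roll against CapaciteTir and apply the GameManager-selected character's damage; death removes the character from team lists and destroys it.
; The first skill only spends the attack and resets highlighted cubes, without any effect.
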(event `self.ReceiveBeginPlay`
  ;[1 1 1] Défini la position du personnage à partir du cube dans lequel il est attaché et défini la couleur
  (`self.SetColor`))

(fn `ActionAttackPerso`
  (params (PersoCible :type "/Game/Projet/Blueprints/Perso Object Reference"))
  (set `self.hasAttaque` false)
  (bind _returnvalue (`GameplayStatics.GetActorOfClass` "/Game/Projet/Blueprints/Vecteur.Vecteur_C"))
  (`/Game/Projet/Blueprints/Vecteur.ResetAllCube` _returnvalue false false true true)
  ;[1 1 1] Touche ?
  (if (< (`KismetMathLibrary.RandomInteger` 100) (`self.CapaciteTir`))
    ;[1 1 1] Inflige des dégâts à l'ennemi
    (bind _returnvalue_2 (`GameplayStatics.GetActorOfClass` "/Game/Projet/Blueprints/GameManager.GameManager_C"))
    (`self.RecoitDegat` PersoCible (`/Game/Projet/Blueprints/Perso.AttackDamage` (`/Game/Projet/Blueprints/GameManager.SelectPerso` _returnvalue_2)))
    (else
      ;[1 1 1] Tir qui rate
      (`KismetSystemLibrary.PrintString` "Fail"))))

(fn `ActionFirstCompetencePerso`
  (params (cubeCible :type "/Game/Projet/Blueprints/Cube Object Reference"))
  (set `self.hasAttaque` false)
  (bind _returnvalue (`GameplayStatics.GetActorOfClass` "/Game/Projet/Blueprints/Vecteur.Vecteur_C"))
  (`/Game/Projet/Blueprints/Vecteur.ResetAllCube` _returnvalue false false true true))

(fn `ActionMovePerso`
  (params (Cube :type "/Game/Projet/Blueprints/Cube Object Reference"))
  (bind _returnvalue (`GameplayStatics.GetActorOfClass` "/Game/Projet/Blueprints/GameManager.GameManager_C"))
  (bind _returnvalue_2 (`GameplayStatics.GetActorOfClass` "/Game/Projet/Blueprints/Vecteur.Vecteur_C"))
  (bind _recupcube (`/Game/Projet/Blueprints/Vecteur.GetCubeFromPerso` _returnvalue_2 self))
  (set `self.NumberMove` (`KismetMathLibrary.FTrunc` (`/Game/Projet/Blueprints/Cube.MoveRange` Cube)))
  (set `/Game/Projet/Blueprints/Cube.Personage` (`/Game/Projet/Blueprints/GameManager.NULLPerso` _returnvalue) _recupcube)
  (set `/Game/Projet/Blueprints/Vecteur.SelectCube` Cube _returnvalue_2)
  (bind _returnvalue_3 (`GameplayStatics.GetActorOfClass` "/Game/Projet/Blueprints/Vecteur.Vecteur_C"))
  (`/Game/Projet/Blueprints/Vecteur.OnMovePerso` _returnvalue_3))

(fn `Death`
  (bind (_returnvalue_x _returnvalue_y) (`KismetMathLibrary.BreakVector` (`self.K2_GetActorLocation` self)))
  (bind _returnvalue (`GameplayStatics.GetActorOfClass` "/Game/Projet/Blueprints/Vecteur.Vecteur_C"))
  (bind _selectennemi (`/Game/Projet/Blueprints/Vecteur.SelectEnnemi` _returnvalue))
  (for _array_element _selectennemi
    (bind (_returnvalue_x_2 _returnvalue_y_2) (`KismetMathLibrary.BreakVector` (`self.K2_GetActorLocation` _array_element)))
    (if (and (== _returnvalue_x_2 (`KismetMathLibrary.Conv_IntToDouble` (`KismetMathLibrary.FTrunc` _returnvalue_x))) (== _returnvalue_y_2 (`KismetMathLibrary.Conv_IntToDouble` (`KismetMathLibrary.FTrunc` _returnvalue_y))))
      (`KismetArrayLibrary.Array_RemoveItem` _selectennemi _array_element)))
  (if (`self.Ennemi`)
    (bind _returnvalue_2 (`GameplayStatics.GetActorOfClass` "/Game/Projet/Blueprints/GameManager.GameManager_C"))
    (`KismetArrayLibrary.Array_RemoveItem` (`/Game/Projet/Blueprints/GameManager.ListEnnemiPerso` _returnvalue_2) self)
    (else
      (bind _returnvalue_3 (`GameplayStatics.GetActorOfClass` "/Game/Projet/Blueprints/GameManager.GameManager_C"))
      (`KismetArrayLibrary.Array_RemoveItem` (`/Game/Projet/Blueprints/GameManager.ListPlayerPerso` _returnvalue_3) self)))
  (`self.K2_DestroyActor`))

(fn `InitStat`
  (bind _lifepoint (`self.LifePoint`))
  (bind _healthbar (`self.HealthBar`))
  (bind _returnvalue (`|CreateWidget` "/Game/Projet/HealthBar/HealthBar.HealthBar_C"))
  (`WidgetComponent.SetWidget` _healthbar _returnvalue)
  (bind _ashealth_bar (cast `/Game/Projet/HealthBar/HealthBar` (`WidgetComponent.GetUserWidgetObject` _healthbar))
    (:`then`
      (bind _output_get (set `self.HealthWidgetREF` _ashealth_bar))
      (set `/Game/Projet/HealthBar/HealthBar.HealthMax` _lifepoint _output_get)
      (bind _output_get_2 (set `self.CurrentLifePoint` _lifepoint))
      (set `/Game/Projet/HealthBar/HealthBar.Health` _output_get_2 _output_get)
      (set `self.NumberMove` (`self.Mvt`)))
    (:`CastFailed`
      (`KismetSystemLibrary.PrintString` "Merde"))))

(fn `MoveToCube`
  (params (ToCube :type "/Game/Projet/Blueprints/Cube Object Reference"))
  (`self.K2_AttachToActor` self ToCube "None" "KeepRelative" "KeepRelative" "KeepRelative" true)
  (`self.K2_SetActorLocation` self (+ (`self.K2_GetActorLocation` ToCube) (0.0 0.0 50.0)) false false)
  (set `/Game/Projet/Blueprints/Cube.Personage` self ToCube))

(fn `RecoitDegat`
  (params (AttackDmg :type "Float (double-precision)"))
  ;[1 1 1] Affiche le nombre de dégâts qu'il reçoit
  (`KismetSystemLibrary.PrintString` (`KismetStringLibrary.Concat_StrStr` "Inflige " (`KismetStringLibrary.Conv_DoubleToString` AttackDmg) " dégâts"))
  ;[1 1 1] Change les points de vie
  (bind _output_get (set `self.CurrentLifePoint` (- (`self.CurrentLifePoint`) AttackDmg)))
  ;[1 1 1] Affiche les points de vie restant
  (bind _output_get_2 (set `/Game/Projet/HealthBar/HealthBar.Health` _output_get (`self.HealthWidgetREF`)))
  (`KismetSystemLibrary.PrintString` (`KismetStringLibrary.Concat_StrStr` "Il reste  " (`KismetStringLibrary.Conv_DoubleToString` _output_get_2) " points de vie"))
  (if (<= (`self.CurrentLifePoint`) 0.0)
    (`self.Death`)))

(fn `SelectColor`
  (params (Select :type Boolean))
  (if Select
    (if (`self.Ennemi`)
      (`PrimitiveComponent.SetMaterial` (`self.Cone`) 0 "/Game/Projet/Material/Yellow.Yellow")
      (else
        (`PrimitiveComponent.SetMaterial` (`self.Cone`) 0 "/Game/Projet/Material/Yellow.Yellow")))
    (elif (`self.Ennemi`)
      (`PrimitiveComponent.SetMaterial` (`self.Cone`) 0 "/Game/Projet/Material/Red.Red")
      (else
        (`PrimitiveComponent.SetMaterial` (`self.Cone`) 0 "/Game/Projet/Material/Blue.Blue")))))

(fn `SetColor`
  (if (`self.Ennemi`)
    (`PrimitiveComponent.SetMaterial` (`self.Cone`) 0 "/Game/Projet/Material/Red.Red")
    (else
      (`PrimitiveComponent.SetMaterial` (`self.Cone`) 0 "/Game/Projet/Material/Blue.Blue"))))

(fn `SetMovePerso`
  (set `self.NumberMove` (`self.Mvt`)))

(fn `UserConstructionScript`
  (`self.SetColor`))

(fn `ZoneAttackPerso`
  (bind _returnvalue (`GameplayStatics.GetActorOfClass` "/Game/Projet/Blueprints/Vecteur.Vecteur_C"))
  (bind _recupcube (`/Game/Projet/Blueprints/Vecteur.GetCubeFromPerso` _returnvalue self))
  (`/Game/Projet/Blueprints/Vecteur.ResetAllCube` _returnvalue false false true true)
  (if (`self.hasAttaque`)
    (`/Game/Projet/Blueprints/Vecteur.OnCreationAttackArea` _returnvalue _recupcube)))

(fn `ZoneFirstCompetencePerso`
  (params (Portee :type Integer))
  (bind _returnvalue (`GameplayStatics.GetActorOfClass` "/Game/Projet/Blueprints/Vecteur.Vecteur_C"))
  (bind _recupcube (`/Game/Projet/Blueprints/Vecteur.GetCubeFromPerso` _returnvalue self))
  (`/Game/Projet/Blueprints/Vecteur.ResetAllCube` _returnvalue false false true true)
  (if (`self.hasAttaque`)
    (`/Game/Projet/Blueprints/Vecteur.CreateArea` _returnvalue Portee _recupcube false false true)))

(fn `ZoneMovePerso`
  (bind _returnvalue (`GameplayStatics.GetActorOfClass` "/Game/Projet/Blueprints/Vecteur.Vecteur_C"))
  (bind _recupcube (`/Game/Projet/Blueprints/Vecteur.GetCubeFromPerso` _returnvalue self))
  (`/Game/Projet/Blueprints/Vecteur.OnClickCube` _returnvalue _recupcube (`self.NumberMove`)))