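; Engineer (Mecano) character of a grid tactics game, a child class that adds its stats, team colours, sounds and tick-driven arm, wheel and laser animations.
; Its first skill heals a target up to max HP.
; Its second marks same-height tiles along adjacent directions, then shoves a stack of characters and debris along that line, resolving barrel explosions and collision damage before raising a barricade on the first tile.
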(event `self.ReceiveBeginPlay`
  (`parent.ReceiveBeginPlay`)
  (if (`self.Ennemi`)
    (`PrimitiveComponent.SetCustomDepthStencilValue` (`self.mecano_Body`) 2)
    (`PrimitiveComponent.SetCustomDepthStencilValue` (`self.mecano_Head`) 2)
    (`PrimitiveComponent.SetCustomDepthStencilValue` (`self.mecano_LeftArm`) 2)
    (`PrimitiveComponent.SetCustomDepthStencilValue` (`self.mecano_RightArm`) 2)
    (`PrimitiveComponent.SetCustomDepthStencilValue` (`self.mecano_Wheels`) 2)
    (else
      (`PrimitiveComponent.SetCustomDepthStencilValue` (`self.mecano_Body`) 1)
      (`PrimitiveComponent.SetCustomDepthStencilValue` (`self.mecano_Head`) 1)
      (`PrimitiveComponent.SetCustomDepthStencilValue` (`self.mecano_LeftArm`) 1)
      (`PrimitiveComponent.SetCustomDepthStencilValue` (`self.mecano_RightArm`) 1)
      (`PrimitiveComponent.SetCustomDepthStencilValue` (`self.mecano_Wheels`) 1))))

(event `self.ReceiveTick`
  (params (DeltaSeconds :type "Float (single-precision)"))
  (`parent.ReceiveTick` DeltaSeconds)
  (if (`self.isAnimationHeal`)
    (`self.AnimationHeal` DeltaSeconds)
    (elif (`self.IsAnimAttack`)
      (`self.AnimationAttack` DeltaSeconds))))

(event `delayHeal`
  (`KismetSystemLibrary.Delay` 0.5)
  (set `self.IsWaitHeal` true))

(fn `ActionAttackPerso`
  (params (PersoCible :type "/Game/Projet/Blueprints/Perso Object Reference"))
  (bind (_returnvalue_x _returnvalue_y) (`KismetMathLibrary.BreakVector` (`SceneComponent.K2_GetComponentLocation` (`/Game/Projet/Blueprints/Perso.Cone` PersoCible))))
  (bind (_returnvalue_x_2 _returnvalue_y_2) (`KismetMathLibrary.BreakVector` (`SceneComponent.K2_GetComponentLocation` (`self.Cone`))))
  (`parent.ActionAttackPerso` PersoCible)
  (set `self.DistanceAB` (- (`KismetMathLibrary.VSize` (- (`KismetMathLibrary.MakeVector` _returnvalue_x _returnvalue_y) (`KismetMathLibrary.MakeVector` _returnvalue_x_2 _returnvalue_y_2))) 50.0))
  (set `self.IsAnimAttack` true)
  (`FMODBlueprintStatics.PlayEvent2D` "/Game/FMOD/Events/Character_SFX/M_Shoot.M_Shoot"))

(fn `ActionFirstCompetencePerso`
  (params (cubeCible :type "/Game/Projet/Blueprints/Cube Object Reference"))
  (bind _personage (`/Game/Projet/Blueprints/Cube.Personage` cubeCible))
  (if (`/Game/Projet/Blueprints/Cube.AllierAttackArea` cubeCible)
    (`/Engine/EditorBlueprintResources/StandardMacros.IsValid` _personage
      (:`Is Valid`
        (bind _isturn (`/Game/Projet/Blueprints/Cube.IsThisPersoTurn` cubeCible _personage))
        (if _isturn
          (`FMODBlueprintStatics.PlayEvent2D` "/Game/FMOD/Events/Character_SFX/M_Repair.M_Repair")
          (`parent.ActionFirstCompetencePerso` cubeCible)
          (`self.Soigne` _personage (`self.Soin`))
          (set `self.isAnimationHeal` true)
          (set `self.IsSecondRotation` false)
          (set `self.IsWaitHeal` false))))))

(fn `ActionSecondCompetencePerso`
  (params (cubeCible :type "/Game/Projet/Blueprints/Cube Object Reference"))
  (locals (NonObstacle :type Boolean :default true) (Compteur :type Integer) (Max :type "Float (double-precision)") (VecteurDirection :type "Vector Structure") (VecteurTemp :type "Vector Structure") (PilePerso :type "Array of /Game/Projet/Blueprints/Perso Object Reference") (ListpersoTMP :type "Array of /Game/Projet/Blueprints/Perso Object Reference") (firstCube :type "/Game/Projet/Blueprints/Cube Object Reference"))
  (bind _vecteurdirection_x (`KismetMathLibrary.BreakVector` (`local.VecteurDirection`)))
  (bind (_vecteurtemp_x _vecteurtemp_y) (`KismetMathLibrary.BreakVector` (`local.VecteurTemp`)))
  (bind _pileperso (`local.PilePerso`))
  (bind (_vecteurtemp_x_2 _vecteurtemp_y_2 _vecteurtemp_z) (`KismetMathLibrary.BreakVector` (`local.VecteurTemp`)))
  (bind _mycube (`self.MyCube`))
  (bind _returnvalue (`KismetMathLibrary.FTrunc` _vecteurtemp_x))
  (bind _returnvalue_2 (`KismetMathLibrary.FTrunc` _vecteurtemp_y))
  (bind _vectory (`/Game/Projet/Blueprints/Cube.VectorY` _mycube))
  (bind _vectorx (`/Game/Projet/Blueprints/Cube.VectorX` _mycube))
  (bind _output (`|GetArrayItem` _pileperso (`KismetArrayLibrary.Array_LastIndex` _pileperso)))
  ;[1 1 1] Vérifie les conditions nécessaires
  (if (`/Game/Projet/Blueprints/Cube.AllierAttackArea` cubeCible)
    ;[1 1 1] Enlève la coloration des cases et considère que l'action d'attaque est terminé
    (`parent.ActionFirstCompetencePerso` cubeCible)
    (set `self.WaitTimeCDComp2` (`self.CDComp2`))
    ;[1 1 1] Initialise la variable max
    (bind _returnvalue_3 (`GameplayStatics.GetActorOfClass` "/Game/Projet/Blueprints/Vecteur.Vecteur_C"))
    (set `local.Max` (`self.Push Comp 2`))
    ;[1 1 1] Défini du vecteur direction + normalize
    (bind _output_get (set `local.VecteurDirection` (`KismetMathLibrary.MakeVector` (`KismetMathLibrary.Conv_IntToDouble` (- (`/Game/Projet/Blueprints/Cube.VectorX` cubeCible) _vectorx)) (`KismetMathLibrary.Conv_IntToDouble` (- (`/Game/Projet/Blueprints/Cube.VectorY` cubeCible) _vectory)))))
    (set `local.VecteurDirection` (`KismetMathLibrary.Normal` _output_get 1.0))
    ;[1 1 1] Définition de la position initiale vecteur temporaire
    (set `local.VecteurTemp` (`KismetMathLibrary.MakeVector` (`KismetMathLibrary.Conv_IntToDouble` _vectorx) (`KismetMathLibrary.Conv_IntToDouble` _vectory) (`KismetMathLibrary.Conv_IntToDouble` (`/Game/Projet/Blueprints/Cube.Hauteur` _mycube))))
    ;[1 1 1] Boucle qui vérifie si on ne recontre pas d'obstacle ou si on ne dépasse pas la portée de charge
    (while (and (`local.NonObstacle`) (< (`local.Compteur`) (`KismetMathLibrary.FTrunc` (`local.Max`))))
      ;[1 1 1] Incrémentation de vecteur temporaire à partir de la direction
      (bind _output_get_2 (set `local.VecteurTemp` (+ (`local.VecteurDirection`) (`local.VecteurTemp`))))
      ;[1 1 1] Récupération du cube
      (bind _cube (`/Game/Projet/Blueprints/Vecteur.GetCubeAtGridPosition` _returnvalue_3 (`KismetMathLibrary.FTrunc` (.x _output_get_2)) (`KismetMathLibrary.FTrunc` (.y _output_get_2))))
      (if (not (!= (`local.Compteur`) 0))
        (set `local.firstCube` _cube))
      ;[1 1 1] Vérifie s'il rencontre des obstacles
      (`/Engine/EditorBlueprintResources/StandardMacros.IsValid` _cube
        (:`Is Valid`
          (if (> (`KismetMathLibrary.Conv_IntToDouble` (`/Game/Projet/Blueprints/Cube.Hauteur` _cube)) _vecteurtemp_z)
            (set `local.NonObstacle` false :!label _label)
            (elif (`/Game/Projet/Blueprints/Cube.isBarriere` _cube)
              (goto _label)
              (else
                (bind _personage (`/Game/Projet/Blueprints/Cube.Personage` _cube))
                ;[1 1 1] Personnage ?
                (`/Engine/EditorBlueprintResources/StandardMacros.IsValid` _personage
                  (:`Is Valid`
                    ;[1 1 1] Baril ou robot ?
                    (if (`/Game/Projet/Blueprints/Perso.IsRobot` _personage)
                      ;[1 1 1] Ajoute +1 à max et ajoute le perso dans la pile
                      (set `local.Max` (+ (`local.Max`) 1.0) :!label _label_2)
                      (`KismetArrayLibrary.Array_AddUnique` (`local.PilePerso`) _personage)
                      (else
                        ;[1 1 1] Cast le baril
                        (bind _asbaril (cast `/Game/Projet/Blueprints/Baril` _personage)
                          (:`then`
                            ;[1 1 1] Vide la liste des personnages qui prendront les dégâts du barils (au cas ou 2 barils sont chargés)
                            (`KismetArrayLibrary.Array_Clear` (`local.ListpersoTMP`))
                            ;[1 1 1] Ajoute à la liste les personnages a portée de l'explosion du baril
                            (bind _listpersovoisin (`/Game/Projet/Blueprints/Baril.GetPersoInRange` _asbaril))
                            (for _array_element _listpersovoisin
                              (`KismetArrayLibrary.Array_AddUnique` (`local.ListpersoTMP`) _array_element))
                            ;[1 1 1] Si il y a des personnages dans la pile, certains sont à portée de l'explosion quand ils sont poussés. Ajouté de manière unique pour eviter qu'un personnage prenne deux fois les dégâts
                            (for (_array_element_2 _array_index) (`local.PilePerso`)
                              (if (<= _array_index (`KismetMathLibrary.FTrunc` (`/Game/Projet/Blueprints/Perso.AttackRange` _asbaril)))
                                (`KismetArrayLibrary.Array_AddUnique` (`local.ListpersoTMP`) _array_element_2)
                                (else
                                  (break))))
                            ;[1 1 1] Inflige les dégâts du baril
                            (for _array_element_3 (`local.ListpersoTMP`)
                              (`self.AccumulDegat` _array_element_3 (`/Game/Projet/Blueprints/Perso.AttackDamage` _asbaril)))
                            ;[1 1 1] Détruit le baril
                            (`self.K2_DestroyActor` _asbaril))
                          (:`CastFailed`
                            (cast `/Game/Projet/Blueprints/Debris` _personage)
                            (goto _label_2))))))
                  (:`Is Not Valid`
                    _))
                ;[1 1 1] +1 au compteur
                (set `local.Compteur` (+ (`local.Compteur`) 1))))))
        (:`Is Not Valid`
          (goto _label))))
    ;[1 1 1] Test si un obstacle a été rencontré
    (if (not (`local.NonObstacle`))
      ;[1 1 1] Obstacle rencontré, le dernier subit les dégâts du mur et on recule le vecteur pour eviter de mettre un personnage dans un mur
      (`/Engine/EditorBlueprintResources/StandardMacros.IsValid` _output
        (:`Is Valid`
          (`self.AccumulDegat` _output 2.0)
          (set `local.VecteurTemp` (- (`local.VecteurTemp`) (`local.VecteurDirection`))))
        (:`Is Not Valid`
          _)))
    ;[1 1 1] Permet de recuperer le perso Null
    (bind _returnvalue_4 (`GameplayStatics.GetActorOfClass` "/Game/Projet/Blueprints/GameManager.GameManager_C"))
    ;[1 1 1] Depile de la pile charge
    (bind (_arrayindex _arrayelement) (`/Engine/EditorBlueprintResources/StandardMacros.ReverseForEachLoop` (`local.PilePerso`))
      (:`LoopBody`
        ;;[1 1 1] seul le deuxième element prend les dégats (l'automate etant le premier)
        (if (== _arrayindex 0)
          (bind _mycube_2 (`/Game/Projet/Blueprints/Perso.MyCube` _arrayelement))
          (`self.AccumulDegat` _arrayelement (`KismetMathLibrary.Conv_IntToDouble` (+ (`KismetMathLibrary.Abs_Int` (- (`/Game/Projet/Blueprints/Cube.VectorX` _mycube_2) _returnvalue)) (`KismetMathLibrary.Abs_Int` (- (`/Game/Projet/Blueprints/Cube.VectorY` _mycube_2) _returnvalue_2))))))
        (set `/Game/Projet/Blueprints/Cube.Personage` (`/Game/Projet/Blueprints/GameManager.NULLPerso` _returnvalue_4) _mycube_2)
        (bind _cube_2 (`/Game/Projet/Blueprints/Vecteur.GetCubeAtGridPosition` _returnvalue_3 _returnvalue _returnvalue_2))
        (set `/Game/Projet/Blueprints/Perso.TargetPushCube` _cube_2 _arrayelement)
        (set `/Game/Projet/Blueprints/Perso.DerHauteur` (`/Game/Projet/Blueprints/Cube.Hauteur` _mycube_2) _arrayelement)
        (set `/Game/Projet/Blueprints/Cube.Personage` _arrayelement _cube_2)
        (set `/Game/Projet/Blueprints/Perso.MyCube` _cube_2 _arrayelement)
        (set `/Game/Projet/Blueprints/Perso.WhereIsPush` (`self.K2_GetActorLocation` _cube_2) _arrayelement)
        (set `/Game/Projet/Blueprints/Perso.IsPushed` true _arrayelement)
        ;;[1 1 1] déplace la position cible
        (set `local.VecteurTemp` (- (`local.VecteurTemp`) (`local.VecteurDirection`))))
      (:`Completed`
        ;[1 1 1] inflige les dégats
        (`/Game/Projet/Blueprints/Vecteur.AllPersoRecoitTmpDegat` _returnvalue_3)
        (`/Game/Projet/Blueprints/Cube.Create Barricade` (`local.firstCube`) _vecteurdirection_x (`self.My_Grey_Material`))
        (`FMODBlueprintStatics.PlayEvent2D` "/Game/FMOD/Events/Character_SFX/M_Wall.M_Wall")))))

(fn `Animation SubitDegat`
  (params (DeltaTime :type "Float (double-precision)"))
  (locals (Mat_Main :type "Material Object Reference"))
  (bind _output_get (set `self.TimerSubit` (- (`self.TimerSubit`) 1)))
  (if (== _output_get 0)
    (set `self.IsAnimSubitDegat` false)
    (bind _returnvalue (`GameplayStatics.GetActorOfClass` "/Game/Projet/Blueprints/Vecteur.Vecteur_C"))
    (if (`self.Ennemi`)
      (set `local.Mat_Main` (`|GetArrayItem` (`/Game/Projet/Blueprints/Vecteur.ColorRedList` _returnvalue)))
      (else
        (set `local.Mat_Main` (`|GetArrayItem` (`/Game/Projet/Blueprints/Vecteur.ColorBlueList` _returnvalue)))))
    (`PrimitiveComponent.SetMaterial` (`self.mecano_Body`) 0 (`local.Mat_Main`))
    (`PrimitiveComponent.SetMaterial` (`self.mecano_Head`) 0 (`local.Mat_Main`))
    (`PrimitiveComponent.SetMaterial` (`self.mecano_WheelsHolder`) 0 (`local.Mat_Main`))
    (else
      (`PrimitiveComponent.SetMaterial` (`self.mecano_Body`) 0 "/Game/Projet/Material/detritus.detritus")
      (`PrimitiveComponent.SetMaterial` (`self.mecano_Head`) 0 "/Game/Projet/Material/detritus.detritus")
      (`PrimitiveComponent.SetMaterial` (`self.mecano_WheelsHolder`) 0 "/Game/Projet/Material/detritus.detritus"))))

(fn `AnimationAttack`
  (params (DeltaSecond :type "Float (double-precision)"))
  (bind _returnvalue (* 300 DeltaSecond))
  (bind _distanceab (`self.DistanceAB`))
  (if (> _distanceab 0.0)
    (`SceneComponent.K2_AddLocalOffset` (`self.laser`) (`KismetMathLibrary.MakeVector` 0.0 (* 200 _returnvalue)) false false)
    (set `self.DistanceAB` (- _distanceab (* 4 _returnvalue)))
    (else
      (set `self.IsAnimAttack` false)
      (`SceneComponent.K2_SetRelativeLocation` (`self.laser`) (0.0 0.0 0.0) false false)
      (`Widget.SetVisibility` (`/Game/Projet/HealthBar/HealthBar.TextBlock_1` (`self.HealthWidgetREF`)) "Hidden"))))

(fn `AnimationHeal`
  (params (DeltaSecond :type "Float (double-precision)"))
  (locals (DeltaSecondLocal :type "Float (double-precision)"))
  (bind _mecano_rightarm (`self.mecano_RightArm`))
  (bind _mecano_rightarm_2 (`self.mecano_RightArm`))
  (bind _returnvalue (* (`local.DeltaSecondLocal`) 200.0))
  (bind _relativerotation_roll (`KismetMathLibrary.BreakRotator` (`SceneComponent.RelativeRotation` (`self.mecano_LeftHand`))))
  (bind (_relativerotation_roll_2 _relativerotation_pitch _relativerotation_yaw) (`KismetMathLibrary.BreakRotator` (`SceneComponent.RelativeRotation` _mecano_rightarm)))
  (bind _relativerotation_roll_3 (`KismetMathLibrary.BreakRotator` (`SceneComponent.RelativeRotation` (`self.mecano_LeftHand`))))
  (bind (_relativerotation_roll_4 _relativerotation_pitch_2 _relativerotation_yaw_2) (`KismetMathLibrary.BreakRotator` (`SceneComponent.RelativeRotation` _mecano_rightarm_2)))
  (set `local.DeltaSecondLocal` DeltaSecond)
  (if (not (`self.IsSecondRotation`))
    (if (> _relativerotation_yaw -90.0)
      (`SceneComponent.K2_AddLocalRotation` _mecano_rightarm (`KismetMathLibrary.MakeRotator` 0.0 0.0 (* (`local.DeltaSecondLocal`) -200.0)) false false)
      (`SceneComponent.K2_AddLocalRotation` (`self.mecano_LeftArm`) (`KismetMathLibrary.MakeRotator` 0.0 0.0 (* (`local.DeltaSecondLocal`) 200.0)) false false)
      (elif (`self.IsWaitHeal`)
        (if (>= _relativerotation_roll 0.0)
          (`SceneComponent.K2_AddLocalRotation` (`self.mecano_RightHand`) (`KismetMathLibrary.MakeRotator` _returnvalue) false false)
          (`SceneComponent.K2_AddLocalRotation` (`self.mecano_LeftHand`) (`KismetMathLibrary.MakeRotator` _returnvalue) false false)
          (else
            (set `self.IsSecondRotation` true)))
        (else
          (`self.delayHeal`))))
    (elif (>= 0.0 _relativerotation_roll_3)
      (`SceneComponent.K2_AddLocalRotation` (`self.mecano_RightHand`) (`KismetMathLibrary.MakeRotator` _returnvalue) false false)
      (`SceneComponent.K2_AddLocalRotation` (`self.mecano_LeftHand`) (`KismetMathLibrary.MakeRotator` _returnvalue) false false)
      (elif (> 0.0 _relativerotation_yaw_2)
        (`SceneComponent.K2_AddLocalRotation` _mecano_rightarm_2 (`KismetMathLibrary.MakeRotator` 0.0 0.0 (* (`local.DeltaSecondLocal`) 100.0)) false false)
        (`SceneComponent.K2_AddLocalRotation` (`self.mecano_LeftArm`) (`KismetMathLibrary.MakeRotator` 0.0 0.0 (* (`local.DeltaSecondLocal`) -100.0)) false false)))))

(fn `AnimationWheel`
  (params (DeltaSecond :type "Float (double-precision)") (`Vitesse Rotation` :type "Float (double-precision)"))
  (`SceneComponent.K2_AddLocalRotation` (`self.mecano_Wheels`) (`KismetMathLibrary.MakeRotator` (* DeltaSecond `Vitesse Rotation`)) false false))

(fn `FallSound`
  (`FMODBlueprintStatics.PlayEvent2D` "/Game/FMOD/Events/Character_SFX/M_Fall.M_Fall"))

(fn `InitStat`
  (bind (_posxj1 _posyj1 _posxj2 _posyj2 _mvt _attackrange _attackdamage _capacitetir _hp _porteesoin _soin _rangecomp2 _pushcomp2 _cdcomp1 _cdcomp2) (break `/Game/Projet/Structure/Structure_Mecano` (make `/Game/Projet/Structure/Structure_Mecano` 1)))
  (set `self.myTypeInt` 2)
  (bind _returnvalue (`GameplayStatics.GetActorOfClass` "/Game/Projet/Blueprints/Vecteur.Vecteur_C"))
  (if (`self.Ennemi`)
    (bind _cube (`/Game/Projet/Blueprints/Vecteur.GetCubeAtGridPosition` _returnvalue _posxj1 _posyj1))
    (set `self.MyCube` _cube)
    (else
      (bind _cube_2 (`/Game/Projet/Blueprints/Vecteur.GetCubeAtGridPosition` _returnvalue _posxj2 _posyj2))
      (set `self.MyCube` _cube_2)))
  (set `self.Mvt` _mvt)
  (set `self.AttackRange` _attackrange)
  (set `self.AttackDamage` _attackdamage)
  (set `self.CapaciteTir` _capacitetir)
  (set `self.LifePoint` _hp)
  (set `self.Portee_Soin` _porteesoin)
  (set `self.Soin` _soin)
  (set `self.Range Comp 2` _rangecomp2)
  (set `self.Push Comp 2` _pushcomp2)
  (set `self.CDComp1` _cdcomp1)
  (set `self.CDComp2` _cdcomp2)
  (set `self.MyMoveTone` 0.0)
  (`parent.InitStat`))

(fn `PlaySoundFall`
  (`FMODBlueprintStatics.PlayEvent2D` "/Game/FMOD/Events/Character_SFX/M_Fall.M_Fall"))

(fn `Set Color`
  (locals (Mat_Main :type "Material Object Reference") (Mat_Shade :type "Material Object Reference") (Mat_Eye :type "Material Object Reference") (Mat_Wheel :type "Material Object Reference") (Mat_Grey :type "Material Object Reference") (Mat_White :type "Material Object Reference"))
  (bind _mecano_rightarm (`self.mecano_RightArm`))
  (bind _mecano_leftarm (`self.mecano_LeftArm`))
  (bind _mecano_wheels (`self.mecano_Wheels`))
  (bind _mecano_body (`self.mecano_Body`))
  (bind _mecano_wheelsholder (`self.mecano_WheelsHolder`))
  (bind _mecano_head (`self.mecano_Head`))
  (bind _returnvalue (`GameplayStatics.GetActorOfClass` "/Game/Projet/Blueprints/Vecteur.Vecteur_C"))
  ;[1 1 1] Verifie l'equipe
  (if (`self.Ennemi`)
    (bind _colorredlist (`/Game/Projet/Blueprints/Vecteur.ColorRedList` _returnvalue))
    ;[1 1 1] Initialisation des couleurs Team Blue
    (set `local.Mat_White` (`|GetArrayItem` _colorredlist 5))
    (set `local.Mat_Grey` (`|GetArrayItem` _colorredlist 4))
    (set `local.Mat_Wheel` (`|GetArrayItem` _colorredlist 3))
    (set `local.Mat_Eye` (`|GetArrayItem` _colorredlist 2))
    (set `local.Mat_Shade` (`|GetArrayItem` _colorredlist 1))
    (set `local.Mat_Main` (`|GetArrayItem` _colorredlist))
    (else
      (bind _colorbluelist (`/Game/Projet/Blueprints/Vecteur.ColorBlueList` _returnvalue))
      ;[1 1 1] Initialisation des couleurs Team Blue
      (set `local.Mat_Main` (`|GetArrayItem` _colorbluelist))
      (set `local.Mat_Shade` (`|GetArrayItem` _colorbluelist 1))
      (set `local.Mat_Eye` (`|GetArrayItem` _colorbluelist 2))
      (set `local.Mat_Wheel` (`|GetArrayItem` _colorbluelist 3))
      (set `local.Mat_Grey` (`|GetArrayItem` _colorbluelist 4))
      (set `local.Mat_White` (`|GetArrayItem` _colorbluelist 5))))
  ;[1 1 1] Couleur du Body
  (`PrimitiveComponent.SetMaterial` _mecano_body 0 (`local.Mat_Main`))
  (`PrimitiveComponent.SetMaterial` _mecano_body 1 (`local.Mat_Shade`))
  (`PrimitiveComponent.SetMaterial` _mecano_body 3 (`local.Mat_Eye`))
  ;[1 1 1] Couleur de Head
  (`PrimitiveComponent.SetMaterial` _mecano_head 0 (`local.Mat_Main`))
  (`PrimitiveComponent.SetMaterial` _mecano_head 1 (`local.Mat_Shade`))
  (`PrimitiveComponent.SetMaterial` _mecano_head 2 (`local.Mat_Grey`))
  (`PrimitiveComponent.SetMaterial` _mecano_head 3 (`local.Mat_Eye`))
  (`PrimitiveComponent.SetMaterial` _mecano_head 4 (`local.Mat_White`))
  ;[1 1 1] Couleur Left Arm
  (`PrimitiveComponent.SetMaterial` _mecano_leftarm 0 (`local.Mat_Shade`))
  (`PrimitiveComponent.SetMaterial` _mecano_leftarm 1 (`local.Mat_Grey`))
  ;[1 1 1] Couleur Right Arm
  (`PrimitiveComponent.SetMaterial` _mecano_rightarm 0 (`local.Mat_Shade`))
  (`PrimitiveComponent.SetMaterial` _mecano_rightarm 1 (`local.Mat_Grey`))
  ;[1 1 1] Couleur Wheels
  (`PrimitiveComponent.SetMaterial` _mecano_wheels 0 (`local.Mat_Wheel`))
  (`PrimitiveComponent.SetMaterial` _mecano_wheels 1 (`local.Mat_Grey`))
  ;[1 1 1] Couleur Hands
  (`PrimitiveComponent.SetMaterial` (`self.mecano_RightHand`) 0 (`local.Mat_Grey`))
  (`PrimitiveComponent.SetMaterial` (`self.mecano_LeftHand`) 0 (`local.Mat_Grey`))
  ;[1 1 1] Couleur Wheels
  (`PrimitiveComponent.SetMaterial` _mecano_wheelsholder 0 (`local.Mat_Main`))
  (`PrimitiveComponent.SetMaterial` _mecano_wheelsholder 1 (`local.Mat_Shade`))
  (`PrimitiveComponent.SetMaterial` _mecano_wheelsholder 2 (`local.Mat_Grey`))
  (`PrimitiveComponent.SetMaterial` (`self.laser`) 0 (`local.Mat_Eye`))
  (set `self.My_Grey_Material` (`local.Mat_Grey`)))

(fn `Soigne`
  (params (persoSoigne :type "/Game/Projet/Blueprints/Perso Object Reference") (Quantite :type "Float (double-precision)"))
  (bind _lifepoint (`/Game/Projet/Blueprints/Perso.LifePoint` persoSoigne))
  (bind _healthwidgetref (`/Game/Projet/Blueprints/Perso.HealthWidgetREF` persoSoigne))
  (bind _returnvalue (+ (`/Game/Projet/Blueprints/Perso.CurrentLifePoint` persoSoigne) Quantite))
  (if (<= _returnvalue _lifepoint)
    (bind _output_get (set `/Game/Projet/Blueprints/Perso.CurrentLifePoint` _returnvalue persoSoigne))
    (set `/Game/Projet/HealthBar/HealthBar.Health` _output_get _healthwidgetref)
    (else
      (bind _output_get_2 (set `/Game/Projet/Blueprints/Perso.CurrentLifePoint` _lifepoint persoSoigne))
      (set `/Game/Projet/HealthBar/HealthBar.Health` _output_get_2 _healthwidgetref))))

(fn `UserConstructionScript`
  (`parent.UserConstructionScript`))

(fn `ZoneFirstCompetencePerso`
  (params (Portee :type "Float (double-precision)"))
  (`parent.ZoneFirstCompetencePerso` (`self.Portee_Soin`)))

(fn `ZoneSecondCompetencePerso`
  (params (Portee :type "Float (double-precision)"))
  (locals (Adjacent :type "Array of Vector Structure"))
  (bind _range_comp_2 (`self.Range Comp 2`))
  (if (== 0 (`self.WaitTimeCDComp2`))
    ;[1 1 1] Recupération du cube d'origine du personnage
    (bind _returnvalue (`GameplayStatics.GetActorOfClass` "/Game/Projet/Blueprints/Vecteur.Vecteur_C"))
    (bind _recupcube (`/Game/Projet/Blueprints/Vecteur.GetCubeFromPerso` _returnvalue self))
    ;[1 1 1] Reset des cases
    (`/Game/Projet/Blueprints/Vecteur.ResetAllCube` _returnvalue false false true true)
    ;[1 1 1] N'a pas lancé son attaque ?
    (if (`self.hasAttaque`)
      ;[1 1 1] Boucle en fonction de la portée
      (for _index (range (+ (`KismetMathLibrary.FTrunc` _range_comp_2) 1))
        ;[1 1 1] Boucle pour les cases adjacents
        (for _array_element (`local.Adjacent`)
          ;[1 1 1] Cherche la case
          (bind _returnvalue_2 (`GameplayStatics.GetActorOfClass` "/Game/Projet/Blueprints/Vecteur.Vecteur_C"))
          (bind _cube (`/Game/Projet/Blueprints/Vecteur.GetCubeAtGridPosition` _returnvalue_2 (+ (`/Game/Projet/Blueprints/Cube.VectorX` _recupcube) (* (`KismetMathLibrary.FTrunc` (.x _array_element)) _index)) (+ (`/Game/Projet/Blueprints/Cube.VectorY` _recupcube) (* (`KismetMathLibrary.FTrunc` (.y _array_element)) _index))))
          (`/Engine/EditorBlueprintResources/StandardMacros.IsValid` _cube
            (:`Is Valid`
              (if (== (`/Game/Projet/Blueprints/Cube.Hauteur` _cube) (`/Game/Projet/Blueprints/Cube.Hauteur` (`self.MyCube`)))
                ;[1 1 1] Applique les modifications
                (set `/Game/Projet/Blueprints/Cube.AllierAttackArea` true _cube)
                (set `/Game/Projet/Blueprints/Cube.MoveRange` (`KismetMathLibrary.Conv_IntToDouble` (- (`KismetMathLibrary.FTrunc` _range_comp_2) _index)) _cube)))))
        (set `/Game/Projet/Blueprints/Cube.AllierAttackArea` false (`self.MyCube`))))
    (else
      (`KismetSystemLibrary.PrintString` "En CD"))))