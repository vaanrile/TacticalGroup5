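; Tank (Char) character for a grid-based tactical game, whose first competence toggles a turret mode.
; InitStat places it on its side's starting cube through the Vecteur grid actor and loads normal and turret stats from the Char structure.
; When the competence targets its own highlighted cube, it swaps movement and attack range, resets NumberMove and stretches or restores its Cone mesh.
; Other overrides just defer to the parent class.
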(event `self.ReceiveBeginPlay`
  (`parent.ReceiveBeginPlay`))

(fn `ActionAttackPerso`
  (params (PersoCible :type "/Game/Projet/Blueprints/Perso Object Reference"))
  (`parent.ActionAttackPerso` PersoCible))

(fn `ActionFirstCompetencePerso`
  (params (cubeCible :type "/Game/Projet/Blueprints/Cube Object Reference"))
  (bind _isturret (`self.IsTurret`))
  (bind _personage (`/Game/Projet/Blueprints/Cube.Personage` cubeCible))
  (if (`/Game/Projet/Blueprints/Cube.AllierAttackArea` cubeCible)
    (`/Engine/EditorBlueprintResources/StandardMacros.IsValid` _personage
      (:`Is Valid`
        (if (== _personage self)
          (`parent.ActionFirstCompetencePerso` cubeCible)
          (set `self.IsTurret` (not _isturret))
          (if _isturret
            (set `self.Mvt` (`self.MvtTurret`))
            (set `self.NumberMove` 0)
            (set `self.AttackRange` (`self.PorteeTurret`))
            (`SceneComponent.SetRelativeScale3D` (`self.Cone`) (0.5 0.5 2.0))
            (else
              (set `self.Mvt` (`self.OriginalMvt`))
              (set `self.NumberMove` 0)
              (set `self.AttackRange` (`self.OriginalPortee`))
              (`SceneComponent.SetRelativeScale3D` (`self.Cone`) (0.5 0.5 0.5)))))))))

(fn `InitStat`
  (bind (_posxj1 _posyj1 _posxj2 _posyj2 _mvt _attackrange _attackdamage _capacitetir _hp _mvtturret _attackrangeturret) (break `/Game/Projet/Structure/Structure_Char` (make `/Game/Projet/Structure/Structure_Char` 1)))
  (bind _returnvalue (`GameplayStatics.GetActorOfClass` "/Game/Projet/Blueprints/Vecteur.Vecteur_C"))
  (if (`self.Ennemi`)
    (bind _cube (`/Game/Projet/Blueprints/Vecteur.GetCubeAtGridPosition` _returnvalue _posxj1 _posyj1))
    (set `self.MyCube` _cube)
    (else
      (bind _cube_2 (`/Game/Projet/Blueprints/Vecteur.GetCubeAtGridPosition` _returnvalue _posxj2 _posyj2))
      (set `self.MyCube` _cube_2)))
  (set `self.Mvt` _mvt)
  (set `self.AttackRange` _attackrange)
  (set `self.AttackDamage` _attackdamage)
  (set `self.CapaciteTir` _capacitetir)
  (set `self.LifePoint` _hp)
  (set `self.MvtTurret` _mvtturret)
  (set `self.PorteeTurret` _attackrangeturret)
  (set `self.OriginalMvt` _mvt)
  (set `self.OriginalPortee` _attackrange)
  (`parent.InitStat`))

(fn `SetColor`
  (`parent.SetColor`))

(fn `UserConstructionScript`
  (`parent.UserConstructionScript`))

(fn `ZoneFirstCompetencePerso`
  (params (Portee :type Integer))
  (`parent.ZoneFirstCompetencePerso` 0))