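; Automate character class for a grid-based tactical game, overriding the parent's first skill with a charge.
; The zone function marks cubes in straight lines along adjacent directions, up to the charge range.
; The action steps along a normalized vector toward an empty target cube, flags higher terrain as an obstacle, damages and stacks characters crossed, each extending the range.
; The nodes that would move the Automate are unconnected.
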(event `self.ReceiveBeginPlay`
  (`parent.ReceiveBeginPlay`))

(fn `ActionAttackPerso`
  (params (PersoCible :type "/Game/Projet/Blueprints/Perso Object Reference"))
  (`parent.ActionAttackPerso` PersoCible))

(fn `ActionFirstCompetencePerso`
  (params (cubeCible :type "/Game/Projet/Blueprints/Cube Object Reference"))
  (locals (NonObstacle :type Boolean :default true) (Compteur :type Integer) (Max :type Integer) (VecteurDirection :type "Vector Structure") (VecteurTemp :type "Vector Structure") (PilePerso :type "Array of /Game/Projet/Blueprints/Perso Object Reference"))
  (bind _mycube (`self.MyCube`))
  (bind _vectory (`/Game/Projet/Blueprints/Cube.VectorY` _mycube))
  (bind _hauteur (`/Game/Projet/Blueprints/Cube.Hauteur` _mycube))
  (bind _vectorx (`/Game/Projet/Blueprints/Cube.VectorX` _mycube))
  (if (`/Game/Projet/Blueprints/Cube.AllierAttackArea` cubeCible)
    (`/Engine/EditorBlueprintResources/StandardMacros.IsValid` (`/Game/Projet/Blueprints/Cube.Personage` cubeCible)
      (:`Is Not Valid`
        (`parent.ActionFirstCompetencePerso` cubeCible)
        (bind _returnvalue (`GameplayStatics.GetActorOfClass` "/Game/Projet/Blueprints/Vecteur.Vecteur_C"))
        (set `local.Max` (`.PorteeCharge_2_F8508C93421B02782E0F3987FF8B5318` (break `/Game/Projet/Structure/AutomateCharge` (make `/Game/Projet/Structure/AutomateCharge` 4))))
        (bind _output_get (set `local.VecteurDirection` (`KismetMathLibrary.MakeVector` (`KismetMathLibrary.Conv_IntToDouble` (- (`/Game/Projet/Blueprints/Cube.VectorX` cubeCible) _vectorx)) (`KismetMathLibrary.Conv_IntToDouble` (- (`/Game/Projet/Blueprints/Cube.VectorY` cubeCible) _vectory)) (`KismetMathLibrary.Conv_IntToDouble` (- (`/Game/Projet/Blueprints/Cube.Hauteur` cubeCible) _hauteur)))))
        (set `local.VecteurDirection` (`KismetMathLibrary.Normal` _output_get))
        (set `local.VecteurTemp` (`KismetMathLibrary.MakeVector` (`KismetMathLibrary.Conv_IntToDouble` _vectorx) (`KismetMathLibrary.Conv_IntToDouble` _vectory) (`KismetMathLibrary.Conv_IntToDouble` _hauteur)))
        (`KismetArrayLibrary.Array_AddUnique` (`local.PilePerso`) self)
        (while (and (`local.NonObstacle`) (<= (`local.Compteur`) (`local.Max`)))
          (bind _output_get_2 (set `local.VecteurTemp` (+ (`local.VecteurDirection`) (`local.VecteurTemp`))))
          (bind _cube (`/Game/Projet/Blueprints/Vecteur.GetCubeAtGridPosition` _returnvalue (`KismetMathLibrary.FTrunc` (.x _output_get_2)) (`KismetMathLibrary.FTrunc` (.y _output_get_2))))
          (`/Engine/EditorBlueprintResources/StandardMacros.IsValid` _cube
            (:`Is Valid`
              (if (> (`KismetMathLibrary.Conv_IntToDouble` (`/Game/Projet/Blueprints/Cube.Hauteur` _cube)) (.z _output_get_2))
                (set `local.NonObstacle` false))
              (bind _personage (`/Game/Projet/Blueprints/Cube.Personage` _cube))
              (`/Engine/EditorBlueprintResources/StandardMacros.IsValid` _personage
                (:`Is Valid`
                  (set `local.Max` (+ (`local.Max`) 1))
                  (`KismetArrayLibrary.Array_AddUnique` (`local.PilePerso`) _personage)
                  (`self.RecoitDegat` _personage 1.0))))))))))

(fn `UserConstructionScript`
  (`parent.UserConstructionScript`))

(fn `ZoneFirstCompetencePerso`
  (params (Portee :type Integer))
  (locals (Adjacent :type "Array of Vector Structure"))
  (bind _porteecharge (break `/Game/Projet/Structure/AutomateCharge` (make `/Game/Projet/Structure/AutomateCharge` 4)))
  ;[1 1 1] Recupération du cube d'origine du personnage
  (bind _returnvalue (`GameplayStatics.GetActorOfClass` "/Game/Projet/Blueprints/Vecteur.Vecteur_C"))
  (bind _recupcube (`/Game/Projet/Blueprints/Vecteur.GetCubeFromPerso` _returnvalue self))
  ;[1 1 1] Reset des cases
  (`/Game/Projet/Blueprints/Vecteur.ResetAllCube` _returnvalue false false true true)
  ;[1 1 1] N'a pas lancé son attaque ?
  (if (`self.hasAttaque`)
    ;[1 1 1] Boucle en fonction de la portée
    (for _index (range (+ _porteecharge 1))
      ;[1 1 1] Boucle pour les cases adjacents
      (for _array_element (`local.Adjacent`)
        ;[1 1 1] Cherche la case
        (bind _returnvalue_2 (`GameplayStatics.GetActorOfClass` "/Game/Projet/Blueprints/Vecteur.Vecteur_C"))
        (bind _cube (`/Game/Projet/Blueprints/Vecteur.GetCubeAtGridPosition` _returnvalue_2 (+ (`/Game/Projet/Blueprints/Cube.VectorX` _recupcube) (* (`KismetMathLibrary.FTrunc` (.x _array_element)) _index)) (+ (`/Game/Projet/Blueprints/Cube.VectorY` _recupcube) (* (`KismetMathLibrary.FTrunc` (.y _array_element)) _index))))
        (`/Engine/EditorBlueprintResources/StandardMacros.IsValid` _cube
          (:`Is Valid`
            ;[1 1 1] Applique les modifications
            (set `/Game/Projet/Blueprints/Cube.AllierAttackArea` true _cube)
            (set `/Game/Projet/Blueprints/Cube.MoveRange` (- _porteecharge _index) _cube)))))))