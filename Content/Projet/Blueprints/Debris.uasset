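; Debris is a non-robot grid piece with life points and no attack, built as a child of a class that provides InitStat.
; InitStat sets those stats, then uses NumberCube (1 to 8) to pick a coordinate pair from a StructureDebris struct.
; The Vecteur actor resolves that pair to MyCube before the parent InitStat runs, which is skipped for any other NumberCube.
; Only the first coordinate pair is explicitly filled in.
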(event `self.ReceiveBeginPlay`
  (`parent.ReceiveBeginPlay`))

(event `self.ReceiveTick`
  (params (DeltaSeconds :type "Float (single-precision)"))
  (`parent.ReceiveTick` DeltaSeconds))

(fn `InitStat`
  (bind _numbercube (`self.numberCube`))
  (bind (_posx1 _posy1 _posx2 _posy2 _posx3 _posy3 _posx4 _posy4 _posx5 _posy5 _posx6 _posy6 _posx7 _posy7 _posx8 _posy8) (break `/Game/Projet/Structure/Structure_Debris` (make `/Game/Projet/Structure/Structure_Debris` 5)))
  (bind _returnvalue (`GameplayStatics.GetActorOfClass` "/Game/Projet/Blueprints/Vecteur.Vecteur_C"))
  (set `self.IsRobot` false)
  (set `self.AttackRange` 0.0)
  (set `self.AttackDamage` 0.0)
  (set `self.LifePoint` 10.0)
  (if (== _numbercube 1)
    (bind _cube (`/Game/Projet/Blueprints/Vecteur.GetCubeAtGridPosition` _returnvalue _posx1 _posy1))
    (set `self.MyCube` _cube)
    (`parent.InitStat` :!label _label)
    (elif (== _numbercube 2)
      (bind _cube_2 (`/Game/Projet/Blueprints/Vecteur.GetCubeAtGridPosition` _returnvalue _posx2 _posy2))
      (set `self.MyCube` _cube_2)
      (goto _label)
      (elif (== _numbercube 3)
        (bind _cube_3 (`/Game/Projet/Blueprints/Vecteur.GetCubeAtGridPosition` _returnvalue _posx3 _posy3))
        (set `self.MyCube` _cube_3)
        (goto _label)
        (elif (== _numbercube 4)
          (bind _cube_4 (`/Game/Projet/Blueprints/Vecteur.GetCubeAtGridPosition` _returnvalue _posx4 _posy4))
          (set `self.MyCube` _cube_4)
          (goto _label)
          (elif (== _numbercube 5)
            (bind _cube_5 (`/Game/Projet/Blueprints/Vecteur.GetCubeAtGridPosition` _returnvalue _posx5 _posy5))
            (set `self.MyCube` _cube_5)
            (goto _label)
            (elif (== _numbercube 6)
              (bind _cube_6 (`/Game/Projet/Blueprints/Vecteur.GetCubeAtGridPosition` _returnvalue _posx6 _posy6))
              (set `self.MyCube` _cube_6)
              (goto _label)
              (elif (== _numbercube 7)
                (bind _cube_7 (`/Game/Projet/Blueprints/Vecteur.GetCubeAtGridPosition` _returnvalue _posx7 _posy7))
                (set `self.MyCube` _cube_7)
                (goto _label)
                (elif (== _numbercube 8)
                  (bind _cube_8 (`/Game/Projet/Blueprints/Vecteur.GetCubeAtGridPosition` _returnvalue _posx8 _posy8))
                  (set `self.MyCube` _cube_8)
                  (goto _label))))))))))

(fn `UserConstructionScript`
  (`parent.UserConstructionScript`))