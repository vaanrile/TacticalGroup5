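; Player camera that becomes the view target on BeginPlay and pans and rotates over an arena.
; Key events set held flags, remapped by a QWERTY/AZERTY switch, which Tick turns into local movement, clamped to arena X/Y bounds, and rotation.
; SetLocationCamera snaps yaw by Face, then Tick overrides manual control, stepping each axis at constant speed to the target.
; BlockInput only clears held flags; smoothed-rotation code is disconnected.
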(event `self.ReceiveBeginPlay`
  (`PlayerController.SetViewTargetWithBlend` (`GameplayStatics.GetPlayerController` 0) self 0.0 "VTBlend_Linear" 0.0 false))

(event `self.ReceiveTick`
  (params (DeltaSeconds :type "Float (single-precision)"))
  (bind _parent (`self.Parent`))
  (bind _speedxlocation (`self.SpeedXLocation`))
  (bind _speedylocation (`self.SpeedYLocation`))
  (bind _parent_2 (`self.Parent`))
  (bind _rightheld (`self.rightHeld`))
  (bind (_templocation_x _templocation_y _templocation_z) (`KismetMathLibrary.BreakVector` (`self.TempLocation`)))
  (bind (_returnvalue_x _returnvalue_y _returnvalue_z) (`KismetMathLibrary.BreakVector` (`SceneComponent.K2_GetComponentLocation` _parent)))
  (bind _returnvalue (* (`self.SpeedZLocation`) 2.0))
  (bind _returnvalue_2 (- _returnvalue_x _templocation_x))
  (bind _returnvalue_3 (- _returnvalue_y _templocation_y))
  (bind _returnvalue_4 (- _returnvalue_z _templocation_z))
  (if (`self.isSmoothCamera`)
    (if (== (`SceneComponent.K2_GetComponentLocation` _parent) (`self.TempLocation`) :`ErrorTolerance` 0.1)
      (set `self.isSmoothCamera` false)
      (else
        (if (and (>= _returnvalue_2 (- 0.0 _speedxlocation)) (<= _returnvalue_2 _speedxlocation))
          (`SceneComponent.K2_SetWorldLocation` _parent (`KismetMathLibrary.MakeVector` _templocation_x _returnvalue_y _returnvalue_z) false false)
          (else
            (`SceneComponent.K2_AddWorldOffset` _parent (`KismetMathLibrary.MakeVector` (* (`self.SpeedXLocation`) (+ (* (`KismetMathLibrary.Conv_BoolToDouble` (< _returnvalue_2 0.0)) 2.0) -1.0))) false false)))
        (if (and (>= _returnvalue_3 (- 0.0 _speedylocation)) (<= _returnvalue_3 _speedylocation))
          (`SceneComponent.K2_SetWorldLocation` _parent (`KismetMathLibrary.MakeVector` _returnvalue_x _templocation_y _returnvalue_z) false false)
          (else
            (`SceneComponent.K2_AddWorldOffset` _parent (`KismetMathLibrary.MakeVector` 0.0 (* (`self.SpeedYLocation`) (+ (* (`KismetMathLibrary.Conv_BoolToDouble` (< _returnvalue_3 0.0)) 2.0) -1.0))) false false)))
        (if (and (>= _returnvalue_4 (- 0.0 _returnvalue)) (<= _returnvalue_4 _returnvalue))
          (`SceneComponent.K2_SetWorldLocation` _parent (`KismetMathLibrary.MakeVector` _returnvalue_x _returnvalue_y _templocation_z) false false)
          (else
            (`SceneComponent.K2_AddWorldOffset` _parent (`KismetMathLibrary.MakeVector` 0.0 0.0 (* (`self.SpeedZLocation`) (+ (* (`KismetMathLibrary.Conv_BoolToDouble` (< _returnvalue_4 0.0)) 2.0) -1.0))) false false)))))
    (else
      (`SceneComponent.K2_AddLocalOffset` (`self.Parent`) (`KismetMathLibrary.MakeVector` (* (- (`KismetMathLibrary.Conv_BoolToDouble` (`self.MoveUpHeld`)) (`KismetMathLibrary.Conv_BoolToDouble` (`self.MoveDownHeld`))) (`self.SpeedXLocation`)) (* (- (`KismetMathLibrary.Conv_BoolToDouble` (`self.MoveRightHeld`)) (`KismetMathLibrary.Conv_BoolToDouble` (`self.MoveLeftHeld`))) (`self.SpeedYLocation`))) false false)
      (`self.LimitCameraCondition`)
      ;[1 1 1] Rotation de la caméra
      (if (`self.leftHeld`)
        (if (not _rightheld)
          (`SceneComponent.K2_AddLocalRotation` _parent_2 (struct :`Yaw` -1.0) false false))
        (elif _rightheld
          (`SceneComponent.K2_AddLocalRotation` _parent_2 (struct :`Yaw` 1.0) false false))))))

(event `Key|A`
  (params (Key :type "Key Structure"))
  (bind _qwerty (`self.QWERTY`))
  (:`Pressed`
    (if _qwerty
      (set `self.MoveLeftHeld` true :!label _label)
      (else
        (set `self.rightHeld` true :!label _label_2))))
  (:`Released`
    (if _qwerty
      (set `self.MoveLeftHeld` false :!label _label_3)
      (else
        (set `self.rightHeld` false :!label _label_4)))))

(event `Key|E`
  (params (Key :type "Key Structure"))
  (bind _qwerty (`self.QWERTY`))
  (:`Pressed`
    (if _qwerty
      (set `self.leftHeld` true)))
  (:`Released`
    (if _qwerty
      (set `self.leftHeld` false))))

(event `Key|Z`
  (params (Key :type "Key Structure"))
  (bind _qwerty (`self.QWERTY`))
  (:`Pressed`
    (if (not _qwerty)
      (set `self.MoveUpHeld` true :!label _label_5)))
  (:`Released`
    (if (not _qwerty)
      (set `self.MoveUpHeld` false :!label _label_6))))

(event `Key|Q`
  (params (Key :type "Key Structure"))
  (bind _qwerty (`self.QWERTY`))
  (:`Pressed`
    (if _qwerty
      (goto _label_2)
      (else
        (goto _label))))
  (:`Released`
    (if _qwerty
      (goto _label_4)
      (else
        (goto _label_3)))))

(event `Key|S`
  (params (Key :type "Key Structure"))
  (:`Pressed`
    (set `self.MoveDownHeld` true))
  (:`Released`
    (set `self.MoveDownHeld` false)))

(event `Key|W`
  (params (Key :type "Key Structure"))
  (bind _qwerty (`self.QWERTY`))
  (:`Pressed`
    (if _qwerty
      (goto _label_5)))
  (:`Released`
    (if _qwerty
      (goto _label_6))))

(event `Key|D`
  (params (Key :type "Key Structure"))
  (:`Pressed`
    (set `self.MoveRightHeld` true))
  (:`Released`
    (set `self.MoveRightHeld` false)))

(fn `BlockInput`
  (set `self.leftHeld` false)
  (set `self.rightHeld` false)
  (set `self.MoveDownHeld` false)
  (set `self.MoveLeftHeld` false)
  (set `self.MoveRightHeld` false)
  (set `self.MoveUpHeld` false))

(fn `LimitCameraCondition`
  (bind _parent (`self.Parent`))
  (bind (_minarena_x _minarena_y) (`KismetMathLibrary.BreakVector2D` (`self.MinArena`)))
  (bind (_maxarena_x _maxarena_y) (`KismetMathLibrary.BreakVector2D` (`self.MaxArena`)))
  (bind (_returnvalue_x _returnvalue_y _returnvalue_z) (`KismetMathLibrary.BreakVector` (`SceneComponent.K2_GetComponentLocation` _parent)))
  ;[1 1 1] X inférieure à la limite minimale ?
  (if (< _returnvalue_x _minarena_x)
    (`SceneComponent.K2_SetWorldLocation` _parent (`KismetMathLibrary.MakeVector` _minarena_x _returnvalue_y _returnvalue_z) false false)
    (else
      ;[1 1 1] X Supérieur à la limite maximale ?
      (if (> _returnvalue_x _maxarena_x)
        (`SceneComponent.K2_SetWorldLocation` _parent (`KismetMathLibrary.MakeVector` _maxarena_x _returnvalue_y _returnvalue_z) false false))))
  ;[1 1 1] Y inférieur à la limite minimal ?
  (if (< _returnvalue_y _minarena_y)
    (`SceneComponent.K2_SetWorldLocation` _parent (`KismetMathLibrary.MakeVector` _returnvalue_x _minarena_y _returnvalue_z) false false)
    (else
      ;[1 1 1] Y Supérieur à la limité maximale
      (if (> _returnvalue_y _maxarena_y)
        (`SceneComponent.K2_SetWorldLocation` _parent (`KismetMathLibrary.MakeVector` _returnvalue_x _maxarena_y _returnvalue_z) false false)))))

(fn `SetLocationCamera`
  (params (Location :type "Vector Structure") (Face :type Boolean))
  (bind _returnvalue (* (- (`KismetMathLibrary.Conv_BoolToDouble` Face) 1.0) 180.0))
  ;[1 1 1] Prévient que l'on va déplacer la caméra
  (set `self.isSmoothCamera` true)
  ;[1 1 1] Stock la position temporairement et la rotation
  (set `self.TempLocation` Location)
  (set `self.TempZRotation` _returnvalue)
  (`SceneComponent.K2_SetWorldRotation` (`self.Parent`) (`KismetMathLibrary.MakeRotator` 0.0 0.0 _returnvalue) false false))

(fn `UserConstructionScript`)