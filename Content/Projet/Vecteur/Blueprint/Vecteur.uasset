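; Grid manager for a tactical game on Cube tiles, handling character placement, movement and range highlights.
; BeginPlay derives each cube's 2D coordinates from this actor's position, indexes them in a dictionary and snaps Perso actors onto them.
; Events flood-fill move, attack and toggleable enemy areas through adjacent cubes, move GameManager's selected character, and clear highlights on turn change.
; A debug K key randomly overheats height-zero cubes, scaled by turn count.
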(event `OnCreationAttackArea`
  (params (Cube :type "/Game/Projet/Cube/Blueprint/Cube Object Reference"))
  (`self.CreateArea` (`/Game/Projet/Perso/Blueprint/Perso.AttackRange` (`/Game/Projet/Cube/Blueprint/Cube.Personage` Cube)) Cube false false true)
  (`self.ResetAllCube` false))

(event `TurnChange`
  (`KismetArrayLibrary.Array_Clear` (`self.SelectEnnemi`))
  (`self.ResetAllCube` true true true))

(event `CheckEnnemiRadius`
  (params (PersoClick :type "/Game/Projet/Cube/Blueprint/Cube Object Reference"))
  (bind _selectennemi (`self.SelectEnnemi`))
  ;[1 1 1] Vérifie si le cube sélectionné est dans la liste
  (if (`KismetArrayLibrary.Array_Contains` _selectennemi PersoClick)
    ;[1 1 1] Enlève
    (`KismetArrayLibrary.Array_RemoveItem` _selectennemi PersoClick)
    (else
      ;[1 1 1] Ajoute
      (`KismetArrayLibrary.Array_AddUnique` _selectennemi PersoClick)))
  ;[1 1 1] Réinitialise la zone d'ennemi
  (`self.ResetAllCube` true)
  ;[1 1 1] Recréer la zone d'ennemi
  (for _array_element (`self.SelectEnnemi`)
    (`self.CreateArea` (`/Game/Projet/Perso/Blueprint/Perso.NumberMove` (`/Game/Projet/Cube/Blueprint/Cube.Personage` _array_element)) _array_element true)
    (`self.ResetAllCube` false)))

(event `OnMovePerso`
  (bind _selectcube (`self.SelectCube`))
  (bind _returnvalue (`GameplayStatics.GetActorOfClass` "/Game/Projet/GameManager/Blueprint/GameManager.GameManager_C"))
  (bind _selectperso (`/Game/Projet/GameManager/Blueprint/GameManager.SelectPerso` _returnvalue))
  (`self.K2_AttachToActor` _selectperso _selectcube "None" "KeepRelative" "KeepRelative" "KeepRelative" true)
  (`self.K2_SetActorLocation` _selectperso (+ (`self.K2_GetActorLocation` _selectcube) (0.0 0.0 50.0)) false false)
  (bind _returnvalue_2 (`GameplayStatics.GetActorOfClass` "/Game/Projet/GameManager/Blueprint/GameManager.GameManager_C"))
  (set `/Game/Projet/Cube/Blueprint/Cube.Personage` (`/Game/Projet/GameManager/Blueprint/GameManager.SelectPerso` _returnvalue_2) (`self.SelectCube`))
  (set `/Game/Projet/GameManager/Blueprint/GameManager.SelectPerso` (`/Game/Projet/GameManager/Blueprint/GameManager.NULLPerso` _returnvalue_2) _returnvalue_2))

(event `OnClickCube`
  (params (CubeSelect :type "/Game/Projet/Cube/Blueprint/Cube Object Reference"))
  (`self.IntermediateCondition` CubeSelect)
  (`self.ConstructAreaMove`))

(event `self.ReceiveBeginPlay`
  ;[1 1 1] Set information for all the cube about a 2D vector
  ;;[1 1 1] Positionne l'objet dans le cube parent
  (`self.K2_SetActorLocation` (`self.K2_GetActorLocation` (`self.GetAttachParentActor`)))
  ;;[1 1 1] Défini les variables vecteurs dans tous les cubes
  (bind _outactors (`GameplayStatics.GetAllActorsOfClass` "/Game/Projet/Cube/Blueprint/Cube.Cube_C"))
  (`self.SetVectorXY` _outactors)
  ;;[1 1 1] Initialize dictionnary
  (for _array_element _outactors
    (`BlueprintMapLibrary.Map_Add` (`self.CubeDictionnary`) (make `IntVector` (`/Game/Projet/Cube/Blueprint/Cube.VectorX` _array_element) (`/Game/Projet/Cube/Blueprint/Cube.VectorY` _array_element)) _array_element))
  (bind _outactors_2 (`GameplayStatics.GetAllActorsOfClass` "/Game/Projet/Perso/Blueprint/Perso.Perso_C"))
  (`self.SetPersoLocation` _outactors_2))

(event `Key|K`
  (params (Key :type "Key Structure"))
  (:`Pressed`
    (`KismetSystemLibrary.PrintString` "Hello")
    (bind _returnvalue (`GameplayStatics.GetActorOfClass` "/Game/Projet/GameManager/Blueprint/GameManager.GameManager_C"))
    (`KismetSystemLibrary.PrintString` "Hello")
    (for _ (range (+ (`/Game/Projet/GameManager/Blueprint/GameManager.NbTour` _returnvalue) 1))
      (`self.CaseSurchauffe`))))

(fn `AnalyseIfPersoInCube`
  (bind _output_get (set `self.SelectCube` null)))

(fn `CaseSurchauffe`
  (bind _cube (`self.GetCubeAtGridPosition` (`KismetMathLibrary.RandomInteger` 16) (`KismetMathLibrary.RandomInteger` 16)))
  (`KismetSystemLibrary.PrintString` "Hello")
  (if (== (`/Game/Projet/Cube/Blueprint/Cube.Hauteur` _cube) 0)
    (set `/Game/Projet/Cube/Blueprint/Cube.Surchauffe` 1 _cube)))

(fn `ConstructAreaMove`
  (bind _outactors (`GameplayStatics.GetAllActorsOfClass` "/Game/Projet/Cube/Blueprint/Cube.Cube_C"))
  (for _array_element _outactors
    (if (not (and (== (`/Game/Projet/Cube/Blueprint/Cube.VectorX` _array_element) (`/Game/Projet/Cube/Blueprint/Cube.VectorX` (`self.SelectCube`))) (== (`/Game/Projet/Cube/Blueprint/Cube.VectorY` _array_element) (`/Game/Projet/Cube/Blueprint/Cube.VectorY` (`self.SelectCube`)))))
      (set `/Game/Projet/Cube/Blueprint/Cube.AllierMoveArea` false _array_element)
      (set `/Game/Projet/Cube/Blueprint/Cube.MoveRange` 0 _array_element)))
  (bind _output_get (set `self.TabCube` (`|MakeArray`)))
  (`KismetArrayLibrary.Array_AddUnique` _output_get (`self.SelectCube`))
  (for _index (range (`/Game/Projet/Cube/Blueprint/Cube.MoveRange` (`self.SelectCube`)))
    (for _array_element_2 (`self.TabCube`)
      (if (== (`/Game/Projet/Cube/Blueprint/Cube.MoveRange` _array_element_2) (- (`/Game/Projet/Cube/Blueprint/Cube.MoveRange` (`self.SelectCube`)) _index))
        (`self.BoucleCheckAdjacent` _outactors _array_element_2 _index)))))

(fn `CreateArea`
  (params (NumberMove :type Integer) (Origin :type "/Game/Projet/Cube/Blueprint/Cube Object Reference") (AreaEnnemiMove :type Boolean) (AreaMove :type Boolean) (AreaAttack :type Boolean))
  (locals (UseCube :type "Array of /Game/Projet/Cube/Blueprint/Cube Object Reference") (StockCube :type "Array of /Game/Projet/Cube/Blueprint/Cube Object Reference") (TempOffset :type "Array of Vector Structure"))
  (bind _usecube (`local.UseCube`))
  (bind _stockcube (`local.StockCube`))
  (bind _origin (`local.Origin`))
  (`KismetArrayLibrary.Array_AddUnique` (`local.UseCube`) Origin)
  (if (`local.AreaMove`)
    (set `/Game/Projet/Cube/Blueprint/Cube.AllierMoveArea` true _origin)
    (set `/Game/Projet/Cube/Blueprint/Cube.MoveRange` NumberMove _origin :!label _label)
    (for _index (range (+ NumberMove 1))
      (for _array_element _usecube
        (for _array_element_2 (`local.TempOffset`)
          (bind _cube (`self.GetCubeAtGridPosition` (+ (`KismetMathLibrary.FTrunc` (.x _array_element_2)) (`/Game/Projet/Cube/Blueprint/Cube.VectorX` _array_element)) (+ (`KismetMathLibrary.FTrunc` (.y _array_element_2)) (`/Game/Projet/Cube/Blueprint/Cube.VectorY` _array_element))))
          (`/Engine/EditorBlueprintResources/StandardMacros.IsValid` _cube
            (:`Is Valid`
              (bind _returnvalue (- NumberMove _index))
              (if (> _returnvalue 0)
                (if (`local.AreaMove`)
                  (set `/Game/Projet/Cube/Blueprint/Cube.AllierMoveArea` true _cube)
                  (set `/Game/Projet/Cube/Blueprint/Cube.MoveRange` _returnvalue _cube :!label _label_2)
                  (`KismetArrayLibrary.Array_AddUnique` (`local.StockCube`) _cube)
                  (elif (`local.AreaAttack`)
                    (set `/Game/Projet/Cube/Blueprint/Cube.AllierAttackArea` true _cube)
                    (goto _label_2)
                    (elif (`local.AreaEnnemiMove`)
                      (set `/Game/Projet/Cube/Blueprint/Cube.EnnemiAttackArea` true _cube)
                      (goto _label_2)))))))))
      (`KismetArrayLibrary.Array_Clear` _usecube)
      (`KismetArrayLibrary.Array_Append` _usecube _stockcube)
      (`KismetArrayLibrary.Array_Clear` _stockcube))
    (elif (`local.AreaAttack`)
      (set `/Game/Projet/Cube/Blueprint/Cube.AllierAttackArea` true _origin)
      (goto _label)
      (elif (`local.AreaEnnemiMove`)
        (set `/Game/Projet/Cube/Blueprint/Cube.EnnemiAttackArea` true _origin)
        (goto _label)))))

(fn `GetCubeAtGridPosition`
  (params (x :type Integer) (y :type Integer))
  (returns (Cube :type "/Game/Projet/Cube/Blueprint/Cube Object Reference"))
  (return (`BlueprintMapLibrary.Map_Find` (`self.CubeDictionnary`) (make `IntVector` x y))))

(fn `IntermediateCondition`
  (params (SelectCube :type "/Game/Projet/Cube/Blueprint/Cube Object Reference"))
  (bind _output_get (set `self.SelectCube` SelectCube))
  (`/Engine/EditorBlueprintResources/StandardMacros.IsValid` (`/Game/Projet/Cube/Blueprint/Cube.Personage` _output_get)
    (:`Is Valid`
      (bind _personage (`/Game/Projet/Cube/Blueprint/Cube.Personage` _output_get))
      (set `/Game/Projet/Cube/Blueprint/Cube.MoveRange` (`/Game/Projet/Perso/Blueprint/Perso.NumberMove` _personage) _output_get)
      (set `/Game/Projet/Cube/Blueprint/Cube.AllierMoveArea` true _output_get)
      (bind _returnvalue (`GameplayStatics.GetActorOfClass` "/Game/Projet/GameManager/Blueprint/GameManager.GameManager_C"))
      (set `/Game/Projet/GameManager/Blueprint/GameManager.SelectPerso` _personage _returnvalue))))

(fn `ResetAllCube`
  (params (IsAreaEnnemiMove :type Boolean) (IsAllierAreaMove :type Boolean) (IsAllierAreaAttack :type Boolean))
  (locals (IsAreaEnnemiMoveVar :type Boolean) (IsAllierAreaMoveVar :type Boolean) (IsAllierAreaAttackVar :type Boolean))
  (set `local.IsAreaEnnemiMoveVar` IsAreaEnnemiMove)
  (set `local.IsAllierAreaMoveVar` IsAllierAreaMove)
  (set `local.IsAllierAreaAttackVar` IsAllierAreaAttack)
  (bind _outactors (`GameplayStatics.GetAllActorsOfClass` "/Game/Projet/Cube/Blueprint/Cube.Cube_C"))
  (for _array_element _outactors
    (set `/Game/Projet/Cube/Blueprint/Cube.MoveRange` 0 _array_element)
    (if (`local.IsAreaEnnemiMoveVar`)
      (set `/Game/Projet/Cube/Blueprint/Cube.EnnemiAttackArea` false _array_element))
    (if (`local.IsAllierAreaMoveVar`)
      (set `/Game/Projet/Cube/Blueprint/Cube.AllierMoveArea` false _array_element))
    (if (`local.IsAllierAreaAttackVar`)
      (set `/Game/Projet/Cube/Blueprint/Cube.AllierAttackArea` false _array_element))))

(fn `SetPersoLocation`
  (params (ListPerso :type "Array of /Game/Projet/Perso/Blueprint/Perso Object Reference"))
  (bind (_returnvalue_x _returnvalue_y) (`KismetMathLibrary.BreakVector` (`self.K2_GetActorLocation`)))
  (bind _cubedictionnary (`self.CubeDictionnary`))
  (for _array_element ListPerso
    (bind (_returnvalue_x_2 _returnvalue_y_2) (`KismetMathLibrary.BreakVector` (`self.K2_GetActorLocation` _array_element)))
    (bind (_returnvalue_x_3 _returnvalue_y_3) (`KismetMathLibrary.BreakVector` (`SceneComponent.K2_GetComponentScale` (`Actor.RootComponent` _array_element))))
    (bind (_min _max) (`StaticMeshComponent.GetLocalBounds` (`/Game/Projet/Perso/Blueprint/Perso.Cone` _array_element)))
    (bind _returnvalue (* (`self.CalculVector` _returnvalue_x_2 _returnvalue_x (* (* _returnvalue_x_3 (- (.x _max) (.x _min))) -1.0)) -1))
    (bind _returnvalue_2 (`self.CalculVector` _returnvalue_y_2 _returnvalue_y (* _returnvalue_y_3 (- (.y _max) (.y _min)))))
    (if (`BlueprintMapLibrary.Map_Contains` _cubedictionnary (make `IntVector` _returnvalue _returnvalue_2))
      (bind _value (`BlueprintMapLibrary.Map_Find` _cubedictionnary (make `IntVector` _returnvalue _returnvalue_2)))
      (`self.K2_SetActorLocation` _array_element (+ (`SceneComponent.K2_GetComponentLocation` (`/Game/Projet/Cube/Blueprint/Cube.DefaultSceneRoot` _value)) (0.0 0.0 50.0)) false false)
      (set `/Game/Projet/Cube/Blueprint/Cube.Personage` _array_element _value))))

(fn `SetVectorXY`
  (params (Array :type "Array of /Game/Projet/Cube/Blueprint/Cube Object Reference"))
  (bind (_returnvalue_x _returnvalue_y) (`KismetMathLibrary.BreakVector` (`self.K2_GetActorLocation`)))
  ;[1 1 1] Boucle qui compare les positions des cubes afin d'y mettre les coordonées de vecteurs 2D
  (for _array_element Array
    (bind (_returnvalue_x_2 _returnvalue_y_2) (`KismetMathLibrary.BreakVector` (`self.K2_GetActorLocation` _array_element)))
    (bind (_returnvalue_x_3 _returnvalue_y_3) (`KismetMathLibrary.BreakVector` (`SceneComponent.K2_GetComponentScale` (`/Game/Projet/Cube/Blueprint/Cube.Cube` _array_element))))
    (bind (_min _max) (`StaticMeshComponent.GetLocalBounds` (`/Game/Projet/Cube/Blueprint/Cube.Cube` _array_element)))
    (set `/Game/Projet/Cube/Blueprint/Cube.VectorX` (* (`self.CalculVector` _returnvalue_x_2 _returnvalue_x (* (* _returnvalue_x_3 (- (.x _max) (.x _min))) -1.0)) -1) _array_element)
    (set `/Game/Projet/Cube/Blueprint/Cube.VectorY` (`self.CalculVector` _returnvalue_y_2 _returnvalue_y (* _returnvalue_y_3 (- (.y _max) (.y _min)))) _array_element)))

(fn `UserConstructionScript`)